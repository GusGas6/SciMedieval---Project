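; BP_SpinHammer is a weapon actor that spins a Greatsword component on demand through HammerSpin and HammerStopSpin events.
; HammerSpin shows the sword and plays a timeline that lerps the RotatingMovement yaw rate for the spin.
; HammerStopSpin zeroes the rate, restores the sword's relative rotation and stops the timeline.
; Paired DoOnce gates make start and stop alternate, with each spin re-arming the stop and vice versa.
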(event `HammerSpin`
  (`/Engine/EditorBlueprintResources/StandardMacros.DoOnce` false :!label _label
    (:`Completed`
      (`SceneComponent.SetVisibility` (`self.Greatsword`) true false)
      (`|ExecutionSequence`
        (:`then_0`
          (`KismetSystemLibrary.DelayUntilNextTick`)
          (bind (_direction _newtrack_0) (`Timeline|Timeline` :!via `PlayFromStart` :!label _label_2)
            (:`Update`
              (set `RotatingMovementComponent.RotationRate` (`KismetMathLibrary.RLerp` (struct) (struct :`Pitch` 2000.0) _newtrack_0) (`self.RotatingMovement`)))))
        (:`then_1`
          (goto _label_3 :!via `Reset`))
        (:`then_2`
          (`SceneComponent.K2_SetRelativeRotation` (`self.Greatsword`) (struct :`Yaw` 95.0) false false))))))

(event `HammerStopSpin`
  (`/Engine/EditorBlueprintResources/StandardMacros.DoOnce` false :!label _label_3
    (:`Completed`
      (set `RotatingMovementComponent.RotationRate` (struct) (`self.RotatingMovement`))
      (`SceneComponent.K2_SetRelativeRotation` (`self.Greatsword`) (struct :`Yaw` 95.0) false false)
      (`|ExecutionSequence`
        (:`then_0`
          (goto _label_2 :!via `Stop`))
        (:`then_1`
          (goto _label :!via `Reset`))))))

(event `self.ReceiveBeginPlay`
  (set `RotatingMovementComponent.RotationRate` (`self.Rotation Rate`) (`self.RotatingMovement`)))

(fn `UserConstructionScript`)