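; BP_SpinStaffFangs animates a staff's fang model, spinning it and swinging its four fangs open and closed.
; RevUp and RevDown use opposing timelines to drive RotatingMovement yaw rate up or ease it to zero, with RevDown also run just after BeginPlay.
; SplitFangs and UnSplitFangs lerp the fangs' relative rotations through timelines, using paired DoOnce gates that re-arm each other so the two actions alternate.
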(event `self.ReceiveBeginPlay`
  (`KismetSystemLibrary.DelayUntilNextTick`)
  (`self.RevDown`))

(event `RevUp`
  (bind _rotatingmovement (`self.RotatingMovement`))
  (bind (_rotationrate_roll _rotationrate_pitch _rotationrate_yaw) (`KismetMathLibrary.BreakRotator` (`RotatingMovementComponent.RotationRate` _rotatingmovement)))
  (`|ExecutionSequence`
    (:`then_0`
      (bind (_direction _newtrack_0) (`Timeline|Timeline` :!via `PlayFromStart` :!label _label)
        (:`Update`
          (set `RotatingMovementComponent.RotationRate` (`KismetMathLibrary.MakeRotator` 0.0 0.0 (`KismetMathLibrary.Lerp` 0.0 400.0 _newtrack_0)) (`self.RotatingMovement`)))))
    (:`then_1`
      (bind (_direction_2 _newtrack_0_2) (`Timeline|Timeline_0` :!via `Stop` :!label _label_2)
        (:`Update`
          (set `RotatingMovementComponent.RotationRate` (`KismetMathLibrary.MakeRotator` 0.0 0.0 (`KismetMathLibrary.Lerp` _rotationrate_yaw 0.0 _newtrack_0_2)) _rotatingmovement))))))

(event `RevDown`
  (`|ExecutionSequence`
    (:`then_0`
      (goto _label :!via `Stop`))
    (:`then_1`
      (goto _label_2 :!via `PlayFromStart`))))

(event `SplitFangs`
  (`/Engine/EditorBlueprintResources/StandardMacros.DoOnce` false :!label _label_3
    (:`Completed`
      (`|ExecutionSequence`
        (:`then_0`
          (`KismetSystemLibrary.DelayUntilNextTick`)
          (bind (_direction _newtrack_0) (`Timeline|Timeline_1` :!via `PlayFromStart` :!label _label_4)
            (:`Update`
              (`|ExecutionSequence`
                (:`then_0`
                  (`SceneComponent.K2_SetRelativeRotation` (`self.StaffFangSingular1`) (`KismetMathLibrary.RLerp` (struct :`Yaw` -180.0) (struct :`Yaw` -180.0 :`Roll` 60.0) _newtrack_0) false false))
                (:`then_1`
                  (`SceneComponent.K2_SetRelativeRotation` (`self.StaffFangSingular2`) (`KismetMathLibrary.RLerp` (struct) (struct :`Roll` 60.0) _newtrack_0) false false))
                (:`then_2`
                  (`SceneComponent.K2_SetRelativeRotation` (`self.StaffFangSingular3`) (`KismetMathLibrary.RLerp` (struct) (struct :`Roll` 60.0) _newtrack_0) false false))
                (:`then_3`
                  (`SceneComponent.K2_SetRelativeRotation` (`self.StaffFangSingular4`) (`KismetMathLibrary.RLerp` (struct :`Yaw` -180.0) (struct :`Yaw` -180.0 :`Roll` 60.0) _newtrack_0) false false))))))
        (:`then_1`
          (bind (_direction_2 _newtrack_0_2) (`Timeline|Timeline_2` :!via `Stop` :!label _label_5)
            (:`Update`
              (`|ExecutionSequence`
                (:`then_0`
                  (`SceneComponent.K2_SetRelativeRotation` (`self.StaffFangSingular1`) (`KismetMathLibrary.RLerp` (struct :`Yaw` -180.0 :`Roll` 60.0) (struct :`Yaw` -180.0) _newtrack_0_2) false false))
                (:`then_1`
                  (`SceneComponent.K2_SetRelativeRotation` (`self.StaffFangSingular2`) (`KismetMathLibrary.RLerp` (struct :`Roll` 60.0) (struct) _newtrack_0_2) false false))
                (:`then_2`
                  (`SceneComponent.K2_SetRelativeRotation` (`self.StaffFangSingular3`) (`KismetMathLibrary.RLerp` (struct :`Roll` 60.0) (struct) _newtrack_0_2) false false))
                (:`then_3`
                  (`SceneComponent.K2_SetRelativeRotation` (`self.StaffFangSingular4`) (`KismetMathLibrary.RLerp` (struct :`Yaw` -180.0 :`Roll` 60.0) (struct :`Yaw` -180.0) _newtrack_0_2) false false))))))
        (:`then_2`
          (`KismetSystemLibrary.DelayUntilNextTick`)
          (goto _label_6 :!via `Reset`))))))

(event `UnSplitFangs`
  (`/Engine/EditorBlueprintResources/StandardMacros.DoOnce` false :!label _label_6
    (:`Completed`
      (`|ExecutionSequence`
        (:`then_0`
          (goto _label_4 :!via `Stop`))
        (:`then_1`
          (`KismetSystemLibrary.DelayUntilNextTick`)
          (goto _label_5 :!via `PlayFromStart`))
        (:`then_2`
          (`KismetSystemLibrary.DelayUntilNextTick`)
          (goto _label_3 :!via `Reset`))))))

(fn `UserConstructionScript`)