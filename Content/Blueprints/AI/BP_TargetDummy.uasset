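; BP_TargetDummy is a great-sword dummy enemy that reacts to hits, gets shocked and ragdolls on death.
; AnyDamage drains health and stores hit force; lightning amplifies that force and triggers retriggerable shock animations and particles.
; Death spawns a launched physics sword and applies a radial impulse, originating lower for tornado damage.
; Fast-moving dummies damage living dummies by velocity, passing on reduced lightning while shocked, and a box overlap calls the player's ToggleGoomba.
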(event `self.ReceiveActorBeginOverlap`
  (params (OtherActor :type "Actor Object Reference"))
  (bind _returnvalue (`KismetMathLibrary.FClamp` (* (`KismetMathLibrary.VSize` (`SceneComponent.GetComponentVelocity` (`self.SkeletalMesh`))) 0.08) 0.0 100.0))
  (bind _asbp_target_dummy (cast `/Game/Blueprints/AI/BP_TargetDummy` OtherActor))
  (if (`/Game/Blueprints/AI/BP_TargetDummy.DEAD` _asbp_target_dummy)
    _
    (elif (<= _returnvalue 10.0)
      _
      (elif (`self.Shocked`)
        (`GameplayStatics.ApplyDamage` _asbp_target_dummy (/ _returnvalue 5.0) null self "/Game/Blueprints/HeathNDamage/DamageType_Lightning.DamageType_Lightning_C")
        (else
          (`GameplayStatics.ApplyDamage` _asbp_target_dummy _returnvalue null self))))))

(event `Death`
  (bind _skeletalmesh (`self.SkeletalMesh`))
  (bind _forcestorage (`self.ForceStorage`))
  (bind _capsule (`self.Capsule`))
  (bind _returnvalue (* _forcestorage 600.0))
  (bind _returnvalue_2 (* _forcestorage 2000.0))
  (`|ExecutionSequence`
    (:`then_0`
      (`/Engine/EditorBlueprintResources/StandardMacros.DoOnce` false
        (:`Completed`
          (bind _returnvalue_3 (`|SpawnActorFromClass` "/Game/Blueprints/Interactibles/BP_EnemySwordPhysicsObject.BP_EnemySwordPhysicsObject_C" (`SceneComponent.K2_GetComponentToWorld` (`self.StaticMesh`)) "AlwaysSpawn" "MultiplyWithRoot" null null))
          (`PrimitiveComponent.AddImpulse` (`/Game/Blueprints/Interactibles/BP_EnemySwordPhysicsObject.PhysicsSword` _returnvalue_3) (* (`KismetMathLibrary.RandomUnitVectorInConeInDegrees` (`self.GetActorUpVector`) 25.0) (* (`self.ForceStorage`) 2.0)) "None" true)
          (`ActorComponent.K2_DestroyComponent` (`self.StaticMesh`)))))
    (:`then_1`
      (`PrimitiveComponent.SetCollisionObjectType` (`self.SkeletalMesh`) "ECC_PhysicsBody")
      (`PrimitiveComponent.SetSimulatePhysics` _skeletalmesh true)
      (if (== (`GameplayStatics.GetObjectClass` (stale `self.ReceiveAnyDamage` DamageType)) "/Game/Blueprints/HeathNDamage/DamageType_Tornado.DamageType_Tornado_C")
        (bind _returnvalue_4 (`self.K2_GetActorLocation` (stale `self.ReceiveAnyDamage` DamageCauser)))
        (`PhysicsObjectBlueprintLibrary.ApplyRadialImpulse` _skeletalmesh (- _returnvalue_4 (0.0 0.0 1000.0)) _returnvalue _returnvalue_2 "RIF_Constant")
        (else
          (`PhysicsObjectBlueprintLibrary.ApplyRadialImpulse` _skeletalmesh _returnvalue_4 _returnvalue _returnvalue_2 "RIF_Constant")
          (set `self.DEAD` true)
          (`PrimitiveComponent.SetCollisionResponseToChannel` _capsule "ECC_GameTraceChannel2" "ECR_Overlap")
          (`PrimitiveComponent.SetCollisionResponseToChannel` _capsule "ECC_Pawn" "ECR_Overlap"))))))

(event `self.Box.OnComponentBeginOverlap`
  (params (OverlappedComponent :type "PrimitiveComponent Object Reference") (OtherActor :type "Actor Object Reference") (OtherComp :type "PrimitiveComponent Object Reference") (OtherBodyIndex :type Integer) (bFromSweep :type Boolean) (SweepResult :type "HitResult Structure (by ref)"))
  (bind _asfirst_person_character (cast `/Game/Blueprints/FirstPersonCharacter` OtherActor))
  (`/Game/Blueprints/FirstPersonCharacter.ToggleGoomba` _asfirst_person_character self))

(event `self.ReceiveAnyDamage`
  (params (Damage :type "Float (single-precision)") (DamageType :type "DamageType Object Reference") (InstigatedBy :type "Controller Object Reference") (DamageCauser :type "Actor Object Reference"))
  (bind _customhealth (`self.CustomHealth`))
  (bind _skeletalmesh (`self.SkeletalMesh`))
  (bind _skeletalmesh_2 (`self.SkeletalMesh`))
  (bind _returnvalue (== (`GameplayStatics.GetObjectClass` DamageType) "/Game/Blueprints/HeathNDamage/DamageType_Lightning.DamageType_Lightning_C"))
  (if _returnvalue
    (`|ExecutionSequence`
      (:`then_0`
        (set `self.Shocked` true)
        (`KismetSystemLibrary.RetriggerableDelay` (`self.ShockDuration`))
        (set `self.Shocked` false)
        (`|ExecutionSequence`
          (:`then_0`
            (goto _label_2 :!via `Reset`))
          (:`then_1`
            (`ActorComponent.Deactivate` (`self.ParticleSystem`))
            (if (not (<= _customhealth 0.0)) :!label _label
              (`SkeletalMeshComponent.PlayAnimation` _skeletalmesh_2 "/Game/Models/Animations/GreatSwordTest_Mark2/great_sword_idle.great_sword_idle" true)))))
      (:`then_1`
        (`/Engine/EditorBlueprintResources/StandardMacros.DoOnce` false :!label _label_2
          (:`Completed`
            (`ActorComponent.Activate` (`self.ParticleSystem`) false)
            (if (`KismetMathLibrary.RandomBool`)
              (`SkeletalMeshComponent.PlayAnimation` _skeletalmesh "/Game/Models/Animations/GreatSwordTest_Mark2/ElectroIntro.ElectroIntro" true)
              (elif (`KismetMathLibrary.RandomBool`)
                (`SkeletalMeshComponent.PlayAnimation` _skeletalmesh "/Game/Models/Animations/GreatSwordTest_Mark2/ElectroBackward.ElectroBackward" true)
                (else
                  (`SkeletalMeshComponent.PlayAnimation` _skeletalmesh "/Game/Models/Animations/GreatSwordTest_Mark2/ElectroForward.ElectroForward" true)))))))
      (:`then_2`
        (set `self.ForceStorage` (* Damage 20.0))
        (set `self.CustomHealth` (- _customhealth Damage) :!label _label_3)
        (if (<= _customhealth 0.0)
          (`self.Death`)
          (elif (`self.Shocked`)
            _
            (elif (not _returnvalue)
              (`SkeletalMeshComponent.PlayAnimation` _skeletalmesh_2 "/Game/Models/Animations/GreatSwordTest_Mark2/great_sword_impact.great_sword_impact" false)
              (`KismetSystemLibrary.Delay` 1.0)
              (goto _label))))))
    (else
      (set `self.ForceStorage` Damage)
      (goto _label_3))))

(fn `UserConstructionScript`)