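; Enemy AI character that roams to random reachable points at walk or sprint speed, with damage reactions, ragdoll death and dismemberment.
; AnyDamage branches on damage type for shock, freezing, slowdown and gibbing, while fast-moving mesh overlaps damage other pawns.
; Death drops the sword as a physics actor, ragdolls the body, then scales and destroys it after a delay.
; Gib events hide bones and spawn mesh chunks with blood effects.
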(event `self.ReceiveBeginPlay`
  (if (`self.InstantDeath`)
    (`self.Death`)
    (else
      (`self.RandomWalk`))))

(event `RandomWalk`
  (bind _charactermovement (`self.CharacterMovement`))
  (if (not (`self.TargetDummy`))
    (if (not (`self.Frozen`)) :!label _label
      (`|AIMoveTo` self (`NavigationSystemV1.K2_GetRandomReachablePointInRadius` (`self.K2_GetActorLocation`) 5000.0 null null) null 50.0
        (:`OnSuccess`
          (`|ExecutionSequence`
            (:`then_0`
              (`/Engine/EditorBlueprintResources/StandardMacros.DoOnce` false :!label _label_2
                (:`Completed`
                  (set `self.LookingAround` true)
                  (set `CharacterMovementComponent.MaxWalkSpeed` 0.0 (`self.CharacterMovement`))
                  (`KismetSystemLibrary.Delay` 10.0)
                  (goto _label_2 :!via `Reset`))))
            (:`then_1`
              (`KismetSystemLibrary.DelayUntilNextTick`)
              (if (`self.LookingAround`) :!label _label_3
                (`KismetSystemLibrary.Delay` 0.1)
                (goto _label_3)
                (else
                  (`KismetSystemLibrary.Delay` 1.0 :!label _label_4)
                  (if (`self.DEAD`)
                    _
                    (elif (`self.Shocked`)
                      (goto _label_4)
                      (else
                        (`|ExecutionSequence`
                          (:`then_0`
                            (goto _label))
                          (:`then_1`
                            (if (`KismetMathLibrary.RandomBoolWithWeight` 0.5)
                              (set `CharacterMovementComponent.MaxWalkSpeed` (`self.MaxSprintSpeed`) _charactermovement)
                              (goto _label_2)
                              (else
                                (set `CharacterMovementComponent.MaxWalkSpeed` (`self.MaxWalkSpeed`) _charactermovement)
                                (goto _label_2)))))))))))))
        (:`OnFail`
          (goto _label_4))))))

(event `self.ReceiveActorBeginOverlap`
  (params (OtherActor :type "Actor Object Reference"))
  (bind _skeletalmesh (`self.SkeletalMesh`))
  (bind _skeletalmesh_2 (`self.SkeletalMesh`))
  (bind _skeletalmesh_3 (`self.SkeletalMesh`))
  (bind _returnvalue (`KismetMathLibrary.FClamp` (/ (`KismetMathLibrary.VSize` (`SceneComponent.GetComponentVelocity` (`self.SkeletalMesh`))) 6.0) 0.0 300.0))
  (bind _aspawn (cast `Pawn` OtherActor))
  (if (not (<= _returnvalue 10.0))
    (if (`self.Shocked`)
      (`GameplayStatics.ApplyDamage` _aspawn (/ _returnvalue 5.0) null self "/Game/Blueprints/HeathNDamage/DamageType_Lightning.DamageType_Lightning_C")
      (else
        (`GameplayStatics.ApplyDamage` _aspawn _returnvalue null self)))
    (`/Engine/EditorBlueprintResources/StandardMacros.IsValid` _aspawn
      (:`Is Valid`
        (`PrimitiveComponent.SetAllPhysicsLinearVelocity` _skeletalmesh (* (`KismetMathLibrary.GetDirectionUnitVector` (`self.K2_GetActorLocation` _aspawn) (`SceneComponent.K2_GetComponentLocation` _skeletalmesh_3)) (/ (`KismetMathLibrary.VSize` (`SceneComponent.GetComponentVelocity` _skeletalmesh_3)) 6.0)) false))
      (:`Is Not Valid`
        (`PrimitiveComponent.SetAllPhysicsLinearVelocity` _skeletalmesh (* (* (`SceneComponent.GetForwardVector` _skeletalmesh_2) (/ (`KismetMathLibrary.VSize` (`SceneComponent.GetComponentVelocity` _skeletalmesh_2)) 6.0)) -1.0) false)))
    (if (`self.Frozen`)
      (`GameplayStatics.ApplyDamage` self 1.0 null self "/Game/Blueprints/HeathNDamage/DamageType_InstaGib.DamageType_InstaGib_C"))))

(event `Death`
  (bind _skeletalmesh (`self.SkeletalMesh`))
  (bind _capsule (`self.Capsule`))
  (bind _capsulecomponent (`self.CapsuleComponent`))
  (bind _returnvalue (* (`self.ForceStorage`) 600.0))
  (`PrimitiveComponent.SetCollisionEnabled` (`self.SkeletalMesh`) "QueryAndPhysics")
  (set `SkeletalMeshComponent.bPauseAnims` true (`self.SkeletalMesh`))
  (`|ExecutionSequence`
    (:`then_0`
      (`/Engine/EditorBlueprintResources/StandardMacros.DoOnce` false
        (:`Completed`
          (bind _returnvalue_2 (`|SpawnActorFromClass` "/Game/Blueprints/Interactibles/BP_EnemySwordPhysicsObject.BP_EnemySwordPhysicsObject_C" (`SceneComponent.K2_GetComponentToWorld` (`self.StaticMesh`)) "AlwaysSpawn" "MultiplyWithRoot" null (`self.Blunt Weapon`) (`self.Thrown Sword Damage Type`) (`self.BaseGlobalAnimRate`) (`self.ChargedGlobalAnimRate`) (`self.Weapon Size`) (`self.Base Damage Sword`) null))
          (`/Engine/EditorBlueprintResources/StandardMacros.IsValid` _returnvalue_2
            (:`Is Valid`
              (`StaticMeshComponent.SetStaticMesh` (`/Game/Blueprints/Interactibles/BP_EnemySwordPhysicsObject.PhysicsSword` _returnvalue_2) (`StaticMeshComponent.StaticMesh` (`self.StaticMesh`)))
              (`PrimitiveComponent.AddImpulse` (`/Game/Blueprints/Interactibles/BP_EnemySwordPhysicsObject.PhysicsSword` _returnvalue_2) (* (`KismetMathLibrary.RandomUnitVectorInConeInDegrees` (`self.GetActorUpVector`) 25.0) (* (`self.ForceStorage`) 0.8)) "None" true)
              (`ActorComponent.K2_DestroyComponent` (`self.StaticMesh`)))))))
    (:`then_1`
      (`PrimitiveComponent.SetCollisionObjectType` (`self.SkeletalMesh`) "ECC_PhysicsBody")
      (`PrimitiveComponent.SetSimulatePhysics` _skeletalmesh true)
      (`/Engine/EditorBlueprintResources/StandardMacros.IsValid` (stale `self.ReceiveAnyDamage` DamageCauser)
        (:`Is Valid`
          (`PhysicsObjectBlueprintLibrary.ApplyRadialImpulse` _skeletalmesh (`self.K2_GetActorLocation` (stale `self.ReceiveAnyDamage` DamageCauser)) _returnvalue _returnvalue "RIF_Constant"))
        (:`Is Not Valid`
          _))
      (set `self.DEAD` true)
      (`PrimitiveComponent.SetCollisionResponseToChannel` _capsule "ECC_GameTraceChannel2" "ECR_Overlap")
      (`PrimitiveComponent.SetCollisionResponseToChannel` _capsule "ECC_Pawn" "ECR_Overlap"))
    (:`then_2`
      (`PrimitiveComponent.SetCollisionEnabled` _capsulecomponent "NoCollision")
      (`PrimitiveComponent.SetEnableGravity` _capsulecomponent false))
    (:`then_3`
      (`KismetSystemLibrary.Delay` 50.0)
      (bind (_direction _newtrack_0) (`Timeline|Timeline` :!via `PlayFromStart`)
        (:`Update`
          (`SceneComponent.SetWorldScale3D` (`self.SkeletalMesh`) (`KismetMathLibrary.VLerp` (0.0 0.0 0.0) (1.0 1.0 1.0) _newtrack_0)))
        (:`Finished`
          (`self.K2_DestroyActor`))))))

(event `FrozenSolid`
  (bind _skeletalmesh (`self.SkeletalMesh`))
  (bind _charactermovement (`self.CharacterMovement`))
  (bind _skeletalmesh_2 (`self.SkeletalMesh`))
  ;[1 1 1] Frozen
  (`|ExecutionSequence`
    (:`then_0`
      (set `SkeletalMeshComponent.bPauseAnims` true _skeletalmesh_2)
      (`PrimitiveComponent.SetMaterial` _skeletalmesh 0 "/Game/Materials/IceTexture_Mat.IceTexture_Mat")
      (`PrimitiveComponent.SetMaterial` _skeletalmesh 1 "/Game/Materials/IceTexture_Mat.IceTexture_Mat")
      (`PrimitiveComponent.SetMaterial` _skeletalmesh 2 "/Game/Materials/IceTexture_Mat.IceTexture_Mat")
      (`PrimitiveComponent.SetMaterial` _skeletalmesh 3 "/Game/Materials/IceTexture_Mat.IceTexture_Mat")
      (set `CharacterMovementComponent.MaxWalkSpeed` 0.0 _charactermovement)
      (set `self.Frozen` true)
      (`NavMovementComponent.StopActiveMovement` _charactermovement)
      (set `CharacterMovementComponent.GroundFriction` 0.5 _charactermovement))
    (:`then_1`
      (`KismetSystemLibrary.Delay` 0.2)
      (set `SkeletalMeshComponent.bNoSkeletonUpdate` true _skeletalmesh_2))))

(event `self.ReceiveAnyDamage`
  (params (Damage :type "Float (single-precision)") (DamageType :type "DamageType Object Reference") (InstigatedBy :type "Controller Object Reference") (DamageCauser :type "Actor Object Reference"))
  (bind _customhealth (`self.CustomHealth`))
  (bind _skeletalmesh (`self.SkeletalMesh`))
  (bind _charactermovement (`self.CharacterMovement`))
  (bind _charactermovement_2 (`self.CharacterMovement`))
  (bind _returnvalue (`SceneComponent.GetSocketLocation` (`self.SkeletalMesh`) "Spine"))
  (bind _returnvalue_2 (== (`GameplayStatics.GetObjectClass` DamageType) "/Game/Blueprints/HeathNDamage/DamageType_Lightning.DamageType_Lightning_C"))
  (if (== (`GameplayStatics.GetObjectClass` DamageType) "/Game/Blueprints/HeathNDamage/DamageType_RandomGibbing.DamageType_RandomGibbing_C")
    (`self.RandomGibRoulette`)
    (elif (== (`GameplayStatics.GetObjectClass` DamageType) "/Game/Blueprints/HeathNDamage/DamageType_InstaGib.DamageType_InstaGib_C")
      (`|ExecutionSequence`
        (:`then_0`
          (`KismetSystemLibrary.DelayUntilNextTick`)
          (`self.SpawnGibChest`))
        (:`then_1`
          (if (`self.Grabbed`) :!label _label_5
            (bind _asfirst_person_character (cast `/Game/Blueprints/FirstPersonCharacter` (`GameplayStatics.GetPlayerCharacter` 0)))
            (`/Game/Blueprints/FirstPersonCharacter.ClearGrabbedEnemy` _asfirst_person_character))
          (set `self.LatestOriginOfDamage` (`self.K2_GetActorLocation` DamageCauser))
          (if (== (`GameplayStatics.GetObjectClass` DamageType) "/Game/Blueprints/HeathNDamage/DamageType_Melee.DamageType_Melee_C")
            (set `SkeletalMeshComponent.bPauseAnims` true _skeletalmesh)
            (set `MovementComponent.Velocity` (0.0 0.0 0.0) (`self.CharacterMovement`))
            (`KismetSystemLibrary.Delay` 0.0)
            (set `SkeletalMeshComponent.bPauseAnims` false _skeletalmesh))
          (if _returnvalue_2
            (`|ExecutionSequence`
              (:`then_0`
                (set `self.Shocked` true)
                (`KismetSystemLibrary.RetriggerableDelay` (`self.ShockDuration`))
                (set `self.Shocked` false)
                (`|ExecutionSequence`
                  (:`then_0`
                    (goto _label_6 :!via `Reset`))
                  (:`then_1`
                    (`ActorComponent.Deactivate` (`self.ParticleSystem`)))))
              (:`then_1`
                (`/Engine/EditorBlueprintResources/StandardMacros.DoOnce` false :!label _label_6
                  (:`Completed`
                    (`ActorComponent.Activate` (`self.ParticleSystem`) false))))
              (:`then_2`
                (set `self.ForceStorage` Damage :!label _label_7)
                (set `self.CustomHealth` (- _customhealth Damage))
                (if (<= _customhealth 0.0)
                  (if (== (`GameplayStatics.GetObjectClass` DamageType) "/Game/Blueprints/HeathNDamage/DamageType_Ice.DamageType_Ice_C")
                    (`self.FrozenSolid`)
                    (else
                      (if (`self.Frozen`)
                        (set `self.DEAD` true)
                        (`self.SpawnGibWaist`))
                      (`/Engine/EditorBlueprintResources/StandardMacros.DoOnce` false
                        (:`Completed`
                          (`self.Death`)))))))
              (:`then_3`
                (`NavMovementComponent.StopActiveMovement` (`self.CharacterMovement`)))
              (:`then_4`
                (if (== (`GameplayStatics.GetObjectClass` DamageType) "/Game/Blueprints/HeathNDamage/DamageType_Explosive.DamageType_Explosive_C") :!label _label_8
                  (set `self.DEAD` true)
                  (`self.SpawnGibChest`))
                (if (== (`GameplayStatics.GetObjectClass` DamageType) "/Game/Blueprints/HeathNDamage/DamageType_Ice.DamageType_Ice_C")
                  (`|ExecutionSequence`
                    (:`then_0`
                      (`|ExecutionSequence` :!label _label_9
                        (:`then_0`
                          (goto _label_7))
                        (:`then_1`
                          (bind _asfirst_person_character_2 (cast `/Game/Blueprints/FirstPersonCharacter` (`GameplayStatics.GetPlayerCharacter` 0)))
                          (`/Game/Blueprints/FirstPersonCharacter.GlobalSlowdown` _asfirst_person_character_2 false)
                          (if (not _returnvalue_2)
                            (for _ (range 6)
                              (bind _returnvalue_3 (`KismetMathLibrary.MakeRotFromZ` (`KismetMathLibrary.RandomUnitVectorInConeInDegrees` (`KismetMathLibrary.GetDirectionUnitVector` (`SceneComponent.K2_GetComponentLocation` (`/Game/Blueprints/FirstPersonCharacter.HurtBox` _asfirst_person_character_2)) _returnvalue) 10.0)))
                              (`GameplayStatics.SpawnEmitterAtLocation` (`self.Emitter Template`) _returnvalue _returnvalue_3 (1.5 1.5 1.5))
                              (`GameplayStatics.SpawnEmitterAtLocation` "/Game/VFX/Bonuses/P_BulletImpact_Meat.P_BulletImpact_Meat" _returnvalue _returnvalue_3 (0.1 0.1 0.1)))))))
                    (:`then_1`
                      (set `self.MaxWalkSpeed` 75.0)
                      (set `self.MaxSprintSpeed` 450.0)
                      (set `CharacterMovementComponent.MaxWalkSpeed` (`self.MaxSprintSpeed`) _charactermovement_2)
                      (set `CharacterMovementComponent.MaxWalkSpeed` (`self.MaxWalkSpeed`) _charactermovement_2)
                      (`KismetSystemLibrary.RetriggerableDelay` 5.0)
                      (set `self.MaxWalkSpeed` 150.0)
                      (set `self.MaxSprintSpeed` 900.0)
                      (set `CharacterMovementComponent.MaxWalkSpeed` (`self.MaxSprintSpeed`) _charactermovement)
                      (set `CharacterMovementComponent.MaxWalkSpeed` (`self.MaxWalkSpeed`) _charactermovement))
                    (:`then_2`
                      (set `self.Emitter Template` "/Game/VFX/MarketplaceAssets/Realistic_Starter_VFX_Pack_Vol2/Particles/Blood/P_Ice_Splat_Cone.P_Ice_Splat_Cone")))
                  (else
                    (set `self.Emitter Template` "/Game/VFX/MarketplaceAssets/Realistic_Starter_VFX_Pack_Vol2/Particles/Blood/P_Blood_Splat_Cone.P_Blood_Splat_Cone")
                    (goto _label_9)))))
            (else
              (goto _label_8)))))
      (else
        (goto _label_5)))))

(event `GibActorBloodMesh`
  (params (location :type "Vector Structure") (rotation :type "Rotator Structure") (scale :type "Vector Structure") (mesh :type "StaticMesh Object Reference") (ContinuosBlood :type Boolean) (BoneName :type Name))
  (bind _forcestorage (`self.ForceStorage`))
  ;[1 0.09093 0] TODO: When total gibbing occurs, have %chance to leave bigger chunks (arms legs etc)
  (`GameplayStatics.SpawnEmitterAtLocation` "/Game/VFX/MarketplaceAssets/Realistic_Starter_VFX_Pack_Vol2/Particles/Blood/P_Blood_Splat_Cone.P_Blood_Splat_Cone" location (`KismetMathLibrary.RandomRotator` false))
  (bind _returnvalue (`|SpawnActorFromClass` "/Game/Blueprints/GibActors/BP_BaseAI_GibActor.BP_BaseAI_GibActor_C" (`KismetMathLibrary.MakeTransform` location rotation scale) "AlwaysSpawn" "MultiplyWithRoot" null false (`self.Frozen`) null))
  (bind _staticmesh (`/Game/Blueprints/GibActors/BP_BaseAI_GibActor.StaticMesh` _returnvalue))
  (`StaticMeshComponent.SetStaticMesh` _staticmesh mesh)
  (`PrimitiveComponent.AddRadialImpulse` _staticmesh (`self.LatestOriginOfDamage`) (* _forcestorage 600.0) (`KismetMathLibrary.FClamp` (* _forcestorage 2000.0) -300.0 300.0) "RIF_Constant" true)
  (if ContinuosBlood
    (`self.ContinuosBloodSplatter` BoneName)))

(event `ContinuosBloodSplatter`
  (params (BoneName :type Name))
  (bind _headsplatterduration (`self.HeadSplatterDuration`))
  (bind (_returnvalue_location _returnvalue_rotation _returnvalue_scale) (`KismetMathLibrary.BreakTransform` (`SkinnedMeshComponent.GetBoneTransform` (`self.SkeletalMesh`) BoneName "RTS_World")))
  ;[1 1 1] Continuos Blood Splatter
  (if (not (`self.Frozen`))
    (`/Engine/EditorBlueprintResources/StandardMacros.DoOnce` false :!label _label_10
      (:`Completed`
        (set `self.ContinuosSplatter` true)
        (`|ExecutionSequence`
          (:`then_0`
            (if (`self.ContinuosSplatter`) :!label _label_11
              (`GameplayStatics.SpawnEmitterAtLocation` "/Game/VFX/MarketplaceAssets/Realistic_Starter_VFX_Pack_Vol2/Particles/Blood/P_Blood_Splat_Cone_Original.P_Blood_Splat_Cone_Original" _returnvalue_location (`KismetMathLibrary.Conv_VectorToRotator` (`KismetMathLibrary.RandomUnitVectorInConeInDegrees` (`KismetMathLibrary.Conv_RotatorToVector` _returnvalue_rotation) 10.0)) _returnvalue_scale)
              (`KismetSystemLibrary.Delay` (`KismetMathLibrary.RandomFloatInRange` 0.05 0.25))
              (goto _label_11)))
          (:`then_1`
            (`KismetSystemLibrary.Delay` (`KismetMathLibrary.RandomFloatInRange` _headsplatterduration (+ _headsplatterduration 5.0)))
            (set `self.ContinuosSplatter` false)
            (goto _label_10 :!via `Reset`)))))))

(event `SpawnGibHead`
  (bind _skeletalmesh (`self.SkeletalMesh`))
  (bind (_returnvalue_location _returnvalue_rotation _returnvalue_scale) (`KismetMathLibrary.BreakTransform` (`SkinnedMeshComponent.GetBoneTransform` _skeletalmesh "Head" "RTS_World")))
  ;[1 1 1] GibbingSystem
  (if (`self.DEAD`)
    (`/Engine/EditorBlueprintResources/StandardMacros.DoOnce` false
      (:`Completed`
        (`SkinnedMeshComponent.HideBoneByName` _skeletalmesh "Head" "PBO_None")
        (`self.GibActorBloodMesh` _returnvalue_location _returnvalue_rotation _returnvalue_scale "/Game/Models/Gibs/StandardArmor/Head_Gib_S_armor.Head_Gib_S_armor" true "Head")
        (set `self.Beheaded` true)
        (bind _asfirst_person_character (cast `/Game/Blueprints/FirstPersonCharacter` (`GameplayStatics.GetPlayerCharacter` 0)))
        (`/Game/Blueprints/FirstPersonCharacter.CriticalSlowdown` _asfirst_person_character)))))

(event `SpawnGibChest`
  (bind _skeletalmesh (`self.SkeletalMesh`))
  (bind (_returnvalue_location _returnvalue_rotation _returnvalue_scale) (`KismetMathLibrary.BreakTransform` (`SkinnedMeshComponent.GetBoneTransform` _skeletalmesh "Spine2" "RTS_World")))
  ;[1 1 1] GibbingSystem
  (if (`self.DEAD`)
    (`/Engine/EditorBlueprintResources/StandardMacros.DoOnce` false
      (:`Completed`
        (`SkinnedMeshComponent.HideBoneByName` _skeletalmesh "Spine2" "PBO_None")
        (`self.GibActorBloodMesh` _returnvalue_location _returnvalue_rotation _returnvalue_scale "/Game/Models/Gibs/StandardArmor/Chest_Gib_S_Armor.Chest_Gib_S_Armor" false "Spine2")
        (if (`KismetMathLibrary.RandomBoolWithWeight` 0.5)
          (`self.SpawnGibHead`))
        (if (`KismetMathLibrary.RandomBoolWithWeight` 0.5)
          (`self.SpawnGibLowerLeftArm`)
          (`self.SpawnGibLowerLeftLeg`))
        (if (`KismetMathLibrary.RandomBoolWithWeight` 0.5)
          (`self.SpawnGibLowerRightArm`)
          (`self.SpawnGibLowerRightLeg`))
        (if (not (`KismetMathLibrary.RandomBoolWithWeight` 0.5))
          (`self.SpawnGibUpperLeftArm`)
          (`self.SpawnGibUpperLeftLeg`))
        (if (`KismetMathLibrary.RandomBoolWithWeight` 0.5)
          (`self.SpawnGibUpperRightArm`)
          (`self.SpawnGibUpperRightLeg`))))))

(event `SpawnGibWaist`
  (bind _skeletalmesh (`self.SkeletalMesh`))
  (bind (_returnvalue_location _returnvalue_rotation _returnvalue_scale) (`KismetMathLibrary.BreakTransform` (`SkinnedMeshComponent.GetBoneTransform` _skeletalmesh "Hips" "RTS_World")))
  ;[1 1 1] GibbingSystem
  (if (or (`self.DEAD`) (`self.Frozen`))
    (`/Engine/EditorBlueprintResources/StandardMacros.DoOnce` false
      (:`Completed`
        (set `SkeletalMeshComponent.bNoSkeletonUpdate` false (`self.SkeletalMesh`))
        (`SkinnedMeshComponent.HideBoneByName` _skeletalmesh "Hips" "PBO_None")
        (`self.GibActorBloodMesh` _returnvalue_location _returnvalue_rotation _returnvalue_scale "/Game/Models/Gibs/StandardArmor/Waist_Gib_s_armor.Waist_Gib_s_armor" false "Spine2")
        (`self.SpawnGibHead`)
        (`self.SpawnGibLowerLeftArm`)
        (`self.SpawnGibLowerLeftLeg`)
        (`self.SpawnGibLowerRightArm`)
        (`self.SpawnGibLowerRightLeg`)
        (`self.SpawnGibUpperLeftArm`)
        (`self.SpawnGibUpperLeftLeg`)
        (`self.SpawnGibUpperRightArm`)
        (`self.SpawnGibUpperRightLeg`)
        (`self.SpawnGibChest`)
        (`KismetSystemLibrary.DelayUntilNextTick`)
        (set `SkeletalMeshComponent.bNoSkeletonUpdate` false (`self.SkeletalMesh`))))))

(event `SpawnGibUpperLeftLeg`
  (bind _skeletalmesh (`self.SkeletalMesh`))
  (bind (_returnvalue_location _returnvalue_rotation _returnvalue_scale) (`KismetMathLibrary.BreakTransform` (`SkinnedMeshComponent.GetBoneTransform` _skeletalmesh "LeftUpLeg" "RTS_World")))
  ;[1 1 1] GibbingSystem
  (if (`self.DEAD`)
    (`/Engine/EditorBlueprintResources/StandardMacros.DoOnce` false
      (:`Completed`
        (`SkinnedMeshComponent.HideBoneByName` _skeletalmesh "LeftUpLeg" "PBO_None")
        (`self.GibActorBloodMesh` _returnvalue_location _returnvalue_rotation _returnvalue_scale "/Game/Models/Gibs/StandardArmor/UpperLeftLeg_Gib_S_Armor.UpperLeftLeg_Gib_S_Armor" (`KismetMathLibrary.RandomBoolWithWeight` 0.2) "LeftUpLeg")
        (`self.SpawnGibLowerLeftLeg`)))))

(event `SpawnGibLowerLeftLeg`
  (bind _skeletalmesh (`self.SkeletalMesh`))
  (bind (_returnvalue_location _returnvalue_rotation _returnvalue_scale) (`KismetMathLibrary.BreakTransform` (`SkinnedMeshComponent.GetBoneTransform` _skeletalmesh "LeftLeg" "RTS_World")))
  ;[1 1 1] GibbingSystem
  (if (`self.DEAD`)
    (`/Engine/EditorBlueprintResources/StandardMacros.DoOnce` false
      (:`Completed`
        (`SkinnedMeshComponent.HideBoneByName` _skeletalmesh "LeftLeg" "PBO_None")
        (`self.GibActorBloodMesh` _returnvalue_location _returnvalue_rotation _returnvalue_scale "/Game/Models/Gibs/StandardArmor/LowerLeftLeg_Gib_S_armor.LowerLeftLeg_Gib_S_armor" (`KismetMathLibrary.RandomBoolWithWeight` 0.2) "LeftLeg")))))

(event `SpawnGibUpperRightLeg`
  (bind _skeletalmesh (`self.SkeletalMesh`))
  (bind (_returnvalue_location _returnvalue_rotation _returnvalue_scale) (`KismetMathLibrary.BreakTransform` (`SkinnedMeshComponent.GetBoneTransform` _skeletalmesh "RightUpLeg" "RTS_World")))
  ;[1 1 1] GibbingSystem
  (if (`self.DEAD`)
    (`/Engine/EditorBlueprintResources/StandardMacros.DoOnce` false
      (:`Completed`
        (`SkinnedMeshComponent.HideBoneByName` _skeletalmesh "RightUpLeg" "PBO_None")
        (`self.GibActorBloodMesh` _returnvalue_location _returnvalue_rotation _returnvalue_scale "/Game/Models/Gibs/StandardArmor/UpperRightLeg_Gib_S_armor.UpperRightLeg_Gib_S_armor" (`KismetMathLibrary.RandomBoolWithWeight` 0.2) "RightUpLeg")
        (`self.SpawnGibLowerRightLeg`)))))

(event `SpawnGibLowerRightLeg`
  (bind _skeletalmesh (`self.SkeletalMesh`))
  (bind (_returnvalue_location _returnvalue_rotation _returnvalue_scale) (`KismetMathLibrary.BreakTransform` (`SkinnedMeshComponent.GetBoneTransform` _skeletalmesh "RightLeg" "RTS_World")))
  ;[1 1 1] GibbingSystem
  (if (`self.DEAD`)
    (`/Engine/EditorBlueprintResources/StandardMacros.DoOnce` false
      (:`Completed`
        (`SkinnedMeshComponent.HideBoneByName` _skeletalmesh "RightLeg" "PBO_None")
        (`self.GibActorBloodMesh` _returnvalue_location _returnvalue_rotation _returnvalue_scale "/Game/Models/Gibs/StandardArmor/LowerRightLeg_Gib_S_armor.LowerRightLeg_Gib_S_armor" (`KismetMathLibrary.RandomBoolWithWeight` 0.2) "RightLeg")))))

(event `SpawnGibUpperLeftArm`
  (bind _skeletalmesh (`self.SkeletalMesh`))
  (bind (_returnvalue_location _returnvalue_rotation _returnvalue_scale) (`KismetMathLibrary.BreakTransform` (`SkinnedMeshComponent.GetBoneTransform` _skeletalmesh "LeftArm" "RTS_World")))
  ;[1 1 1] GibbingSystem
  (if (`self.DEAD`)
    (`/Engine/EditorBlueprintResources/StandardMacros.DoOnce` false
      (:`Completed`
        (`SkinnedMeshComponent.HideBoneByName` _skeletalmesh "LeftArm" "PBO_None")
        (`self.GibActorBloodMesh` _returnvalue_location _returnvalue_rotation _returnvalue_scale "/Game/Models/Gibs/StandardArmor/UpperLeftArm_Gib_S_Armor.UpperLeftArm_Gib_S_Armor" (`KismetMathLibrary.RandomBoolWithWeight` 0.2) "LeftArm")
        (`self.SpawnGibLowerLeftArm`)))))

(event `SpawnGibLowerLeftArm`
  (bind _skeletalmesh (`self.SkeletalMesh`))
  (bind (_returnvalue_location _returnvalue_rotation _returnvalue_scale) (`KismetMathLibrary.BreakTransform` (`SkinnedMeshComponent.GetBoneTransform` _skeletalmesh "LeftForeArm" "RTS_World")))
  ;[1 1 1] GibbingSystem
  (if (`self.DEAD`)
    (`/Engine/EditorBlueprintResources/StandardMacros.DoOnce` false
      (:`Completed`
        (`SkinnedMeshComponent.HideBoneByName` _skeletalmesh "LeftForeArm" "PBO_None")
        (`self.GibActorBloodMesh` _returnvalue_location _returnvalue_rotation _returnvalue_scale "/Game/Models/Gibs/StandardArmor/LowerLeftArm_Gib_S_Armor.LowerLeftArm_Gib_S_Armor" (`KismetMathLibrary.RandomBoolWithWeight` 0.2) "LeftForeArm")))))

(event `SpawnGibUpperRightArm`
  (bind _skeletalmesh (`self.SkeletalMesh`))
  (bind (_returnvalue_location _returnvalue_rotation _returnvalue_scale) (`KismetMathLibrary.BreakTransform` (`SkinnedMeshComponent.GetBoneTransform` _skeletalmesh "RightArm" "RTS_World")))
  ;[1 1 1] GibbingSystem
  (if (`self.DEAD`)
    (`/Engine/EditorBlueprintResources/StandardMacros.DoOnce` false
      (:`Completed`
        (`SkinnedMeshComponent.HideBoneByName` _skeletalmesh "RightArm" "PBO_None")
        (`self.GibActorBloodMesh` _returnvalue_location _returnvalue_rotation _returnvalue_scale "/Game/Models/Gibs/StandardArmor/UpperRightArm_Gib_S_Armor.UpperRightArm_Gib_S_Armor" (`KismetMathLibrary.RandomBoolWithWeight` 0.2) "RightArm")
        (`self.SpawnGibLowerRightArm`)))))

(event `SpawnGibLowerRightArm`
  (bind _skeletalmesh (`self.SkeletalMesh`))
  (bind (_returnvalue_location _returnvalue_rotation _returnvalue_scale) (`KismetMathLibrary.BreakTransform` (`SkinnedMeshComponent.GetBoneTransform` _skeletalmesh "RightForeArm" "RTS_World")))
  ;[1 1 1] GibbingSystem
  (if (`self.DEAD`)
    (`/Engine/EditorBlueprintResources/StandardMacros.DoOnce` false
      (:`Completed`
        (`SkinnedMeshComponent.HideBoneByName` _skeletalmesh "RightForeArm" "PBO_None")
        (`self.GibActorBloodMesh` _returnvalue_location _returnvalue_rotation _returnvalue_scale "/Game/Models/Gibs/StandardArmor/LowerRightArm_Gib_S_Armor.LowerRightArm_Gib_S_Armor" (`KismetMathLibrary.RandomBoolWithWeight` 0.2) "RightForeArm")))))

(event `GibCalculator`
  (params (HitBoneName :type Name))
  ;[1 1 1] GibbingSystem
  (`KismetSystemLibrary.PrintString` (`KismetStringLibrary.Concat_StrStr` "TRYING TO GIB = = " (`KismetStringLibrary.Conv_NameToString` HitBoneName)))
  (switch `name` HitBoneName
    (:`Head`
      (`self.SpawnGibHead`))
    (:`LeftUpLeg`
      (`self.SpawnGibUpperLeftLeg`))
    (:`LeftLeg`
      (`self.SpawnGibLowerLeftLeg`))
    (:`RightUpLeg`
      (`self.SpawnGibUpperRightLeg`))
    (:`RightLeg`
      (`self.SpawnGibLowerRightLeg`))
    (:`LeftArm`
      (`self.SpawnGibUpperLeftArm`))
    (:`LeftForeArm`
      (`self.SpawnGibLowerLeftArm`))
    (:`RightArm`
      (`self.SpawnGibUpperRightArm`))
    (:`RightForeArm`
      (`self.SpawnGibLowerRightArm`))))

(event `RandomGibRoulette`
  ;[1 1 1] GibbingSystem
  (switch `int` (`KismetMathLibrary.RandomIntegerInRange` 0 10)
    (:`0`
      (`self.GibCalculator` "Head"))
    (:`1`
      (`self.GibCalculator` "LeftUpLeg"))
    (:`2`
      (`self.GibCalculator` "LeftLeg"))
    (:`3`
      (`self.GibCalculator` "RightUpLeg"))
    (:`4`
      (`self.GibCalculator` "RightLeg"))
    (:`5`
      (`self.GibCalculator` "LeftArm"))
    (:`6`
      (`self.GibCalculator` "LeftForeArm"))
    (:`7`
      (`self.GibCalculator` "RightArm"))
    (:`8`
      (`self.GibCalculator` "RightForeArm"))))

(fn `UserConstructionScript`)