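; Explosive frog critter that hops randomly via physics impulses when grounded, with a looping timeline-driven breathing scale.
; Any damage knocks it back; the first hit starts a fuse with trail VFX, rapid hopping and pulsing, then it swells and detonates.
; It leaves a toxic AoE bubble and scorch decal, or frozen ground for the FrostFrog variant.
; Overlapping an AoE bubble damages it, allowing chain reactions.
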(event `self.ReceiveBeginPlay`
  (bind (_returnvalue_roll _returnvalue_pitch _returnvalue_yaw) (`KismetMathLibrary.BreakRotator` (`KismetMathLibrary.RandomRotator` false)))
  (bind _frogmesh (`self.FrogMesh`))
  (bind _returnvalue (`SceneComponent.K2_GetComponentLocation` (`self.FrogMesh`)))
  (`|ExecutionSequence`
    (:`then_0`
      (set `self.WaitBeforeNextAction` (`KismetMathLibrary.RandomFloatInRange` (`self.Min`) (`self.Max`)) :!label _label)
      (`KismetSystemLibrary.Delay` (`self.WaitBeforeNextAction`))
      (bind (_outhit _returnvalue_2) (`KismetSystemLibrary.LineTraceSingleForObjects` _returnvalue (- _returnvalue (0.0 0.0 50.0)) (`|MakeArray` "ObjectTypeQuery1" :!type "EObjectTypeQuery Enum") :!label _label_2))
      (if _returnvalue_2
        (`self.K2_SetActorRotation` (`KismetMathLibrary.MakeRotator` 0.0 0.0 (* _returnvalue_yaw 2.0)))
        (`PrimitiveComponent.AddRadialImpulse` (`self.FrogMesh`) (`SceneComponent.K2_GetComponentLocation` (`self.JumpOrigin`)) (`KismetMathLibrary.RandomFloatInRange` 400.0 800.0) (`KismetMathLibrary.RandomFloatInRange` 400.0 700.0) "RIF_Constant" true)
        (goto _label)
        (else
          (goto _label))))
    (:`then_1`
      (if (not (`self.Detonating`)) :!label _label_3
        (bind (_direction _newtrack_0) (`Timeline|BreathingAnim` :!via `PlayFromStart` :!label _label_4)
          (:`Update`
            (`SceneComponent.SetWorldScale3D` (`self.FrogMesh`) (`KismetMathLibrary.VLerp` (1.0 1.0 1.0) (1.2 1.2 1.2) _newtrack_0)))
          (:`Finished`
            (if (not (`self.AboutToExplode`))
              (set `self.CustomTimeDilation` (`KismetMathLibrary.RandomFloatInRange` 0.8 1.2)))
            (`KismetSystemLibrary.Delay` 0.0)
            (goto _label_3)))))
    (:`then_2`
      (if (`self.FrostFrog`)
        (`PrimitiveComponent.SetMaterial` _frogmesh 0 "/Game/Materials/Frog/FrostFrog_Brown2.FrostFrog_Brown2")
        (`PrimitiveComponent.SetMaterial` _frogmesh 1 "/Game/Materials/Frog/FrostFrog_Brown.FrostFrog_Brown")
        (`NiagaraComponent.SetAsset` (`self.PoisonTrail`) "/Game/VFX/MarketplaceAssets/sA_Megapack_v1/sA_StylizedAttacksPack/FX/NiagaraSystems/NS_CartoonyIceTrail.NS_CartoonyIceTrail" true)))))

(event `self.ReceiveAnyDamage`
  (params (Damage :type "Float (single-precision)") (DamageType :type "DamageType Object Reference") (InstigatedBy :type "Controller Object Reference") (DamageCauser :type "Actor Object Reference"))
  (bind _forcestorage (`self.ForceStorage`))
  (bind _returnvalue (`SceneComponent.K2_GetComponentLocation` (`self.FrogMesh`)))
  (set `self.ForceStorage` Damage)
  (`PhysicsObjectBlueprintLibrary.ApplyRadialImpulse` (`self.FrogMesh`) (`self.K2_GetActorLocation` DamageCauser) (* _forcestorage 2.0) (* _forcestorage 3.0) "RIF_Constant")
  (`/Engine/EditorBlueprintResources/StandardMacros.DoOnce` false
    (:`Completed`
      (set `self.AboutToExplode` true)
      (`|ExecutionSequence`
        (:`then_0`
          (goto _label_4 :!via `Stop`))
        (:`then_1`
          (`ActorComponent.Activate` (`self.PoisonTrail`) true)
          (`KismetSystemLibrary.Delay` (`self.TimeUntilDetonate`))
          (set `self.Detonating` true)
          (`|ExecutionSequence`
            (:`then_0`
              (goto _label_4 :!via `Stop`))
            (:`then_1`
              (`KismetSystemLibrary.DelayUntilNextTick`)
              (bind (_direction _newtrack_0) (`Timeline|DetonateTL` :!via `PlayFromStart`)
                (:`Update`
                  (`SceneComponent.SetWorldScale3D` (`self.FrogMesh`) (`KismetMathLibrary.VLerp` (1.0 1.0 1.0) (2.0 3.0 3.0) _newtrack_0)))
                (:`Finished`
                  (if (`self.FrostFrog`)
                    (bind (_outhit _returnvalue_2) (`KismetSystemLibrary.LineTraceSingleForObjects` (`SceneComponent.K2_GetComponentLocation` (`self.FrogMesh`)) (- (`self.K2_GetActorLocation`) (0.0 0.0 1000.0)) (`|MakeArray` "ObjectTypeQuery1" :!type "EObjectTypeQuery Enum")))
                    (if _returnvalue_2
                      (bind (_bblockinghit _binitialoverlap _time _distance _location _impactpoint _normal) (`GameplayStatics.BreakHitResult` _outhit))
                      (`|SpawnActorFromClass` "/Game/Blueprints/MagicSpells/Ice/BP_FrozenGround.BP_FrozenGround_C" (`KismetMathLibrary.MakeTransform` _location (`KismetMathLibrary.MakeRotFromZ` _normal)) "Undefined" "MultiplyWithRoot" null null))
                    (`NiagaraFunctionLibrary.SpawnSystemAtLocation` "/Game/VFX/Bonuses/P_Poof_Ice.P_Poof_Ice" (`self.K2_GetActorLocation`) (`self.K2_GetActorRotation`))
                    (else
                      (`|SpawnActorFromClass` "/Game/Blueprints/HeathNDamage/BP_AoEBubble.BP_AoEBubble_C" (`KismetMathLibrary.MakeTransform` (`SceneComponent.K2_GetComponentLocation` (`self.FrogMesh`))) "Undefined" "MultiplyWithRoot" null 400.0 200.0 false false 600.0 "/Game/Blueprints/HeathNDamage/DamageType_Explosive.DamageType_Explosive_C" true null)
                      (bind (_outhit_2 _returnvalue_3) (`KismetSystemLibrary.LineTraceSingleForObjects` _returnvalue (- _returnvalue (0.0 0.0 250.0)) (`|MakeArray` "ObjectTypeQuery1" :!type "EObjectTypeQuery Enum")))
                      (if _returnvalue_3
                        (bind (_bblockinghit_2 _binitialoverlap_2 _time_2 _distance_2 _location_2 _impactpoint_2 _normal_2) (`GameplayStatics.BreakHitResult` _outhit_2))
                        (`|SpawnActorFromClass` "/Game/Blueprints/Lighting/BP_ScorchDecal.BP_ScorchDecal_C" (`KismetMathLibrary.MakeTransform` _location_2 (`KismetMathLibrary.MakeRotFromZ` _normal_2) (2.0 2.0 2.0)) "AlwaysSpawn" "MultiplyWithRoot" null null))))
                  (`self.K2_DestroyActor`))))
            (:`then_2`
              (bind (_direction_2 _newtrack_0_2) (`Timeline|Timeline` :!via `Stop` :!label _label_5)
                (:`Update`
                  (`SceneComponent.SetWorldScale3D` (`self.FrogMesh`) (`KismetMathLibrary.VLerp` (0.9 0.9 0.9) (1.3 1.3 1.3) _newtrack_0_2)))
                (:`Finished`
                  (`KismetSystemLibrary.Delay` 0.0)
                  (if (not (`self.Detonating`)) :!label _label_6
                    (goto _label_5 :!via `PlayFromStart`)))))))
        (:`then_2`
          (goto _label_6))
        (:`then_3`
          (set `self.Min` 0.2)
          (set `self.Max` 0.3)
          (`KismetSystemLibrary.DelayUntilNextTick`)
          (goto _label_2))))))

(event `self.ReceiveActorBeginOverlap`
  (params (OtherActor :type "Actor Object Reference"))
  (cast `/Game/Blueprints/HeathNDamage/BP_AoEBubble` OtherActor)
  (`GameplayStatics.ApplyDamage` self 500.0 null OtherActor))

(fn `UserConstructionScript`)