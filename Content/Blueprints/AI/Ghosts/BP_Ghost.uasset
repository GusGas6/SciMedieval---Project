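; BP_Ghost is a roaming ghost that stays invisible until it overlaps BP_FakeLanternLightDecal, which fades in its dynamic materials.
; BeginPlay runs a hover loop, random AIMoveTo roaming and timed mesh height changes that simulate flight over ground navigation.
; Any damage kills it, stopping movement, revealing it and turning it relative to the attacker.
; A separate DeathExplosion event, not called here, shrinks the mesh, spawns sparks and destroys the actor.
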(event `self.ReceiveBeginPlay`
  (bind _ghostmesh (`self.GhostMesh`))
  (bind _ghostmesh_2 (`self.GhostMesh`))
  (bind _ghosthovermover (`self.GhostHoverMover`))
  (bind _ghostmesh_3 (`self.GhostMesh`))
  (bind (_relativelocation_x _relativelocation_y _relativelocation_z) (`KismetMathLibrary.BreakVector` (`SceneComponent.RelativeLocation` (`self.GhostMesh`))))
  (bind _relativelocation (`SceneComponent.RelativeLocation` _ghosthovermover))
  (bind _relativerotation (`SceneComponent.RelativeRotation` _ghosthovermover))
  ;[1 1 1] Beginplay
  (`|ExecutionSequence`
    (:`then_0`
      ;[1 1 1] bASE hOVER
      (`KismetSystemLibrary.MoveComponentTo` _ghosthovermover (+ _relativelocation (0.0 0.0 35.0)) _relativerotation true true 2.0 :!label _label)
      (if (not (`self.Dead`))
        (`KismetSystemLibrary.MoveComponentTo` _ghosthovermover (+ _relativelocation (0.0 0.0 -35.0)) _relativerotation true true 2.0)
        (if (not (`self.Dead`))
          (goto _label))))
    (:`then_1`
      ;[1 1 1] Control Roaming Flying
      (if (not (`self.ForceSameHeight`)) :!label _label_2
        (if (or (< _relativelocation_z -3000.0) (> _relativelocation_z 3000.0) (`self.ForceGroundLevelHeight`)) :!label _label_3
          (set `self.TargetHeight` 0.0)
          (else
            (set `self.TargetHeight` (`KismetMathLibrary.RandomFloatInRange` -2000.0 2000.0))))
        (if (not (or (`self.Dead`) (`self.ChasingPlayer`)))
          (bind (_direction _newtrack_0) (`Timeline|Fly` :!via `PlayFromStart` :!label _label_4)
            (:`Update`
              (`SceneComponent.K2_SetRelativeLocation` _ghostmesh_3 (`KismetMathLibrary.VLerp` (`SceneComponent.RelativeLocation` _ghostmesh_3) (`KismetMathLibrary.MakeVector` 0.0 0.0 (`self.TargetHeight`)) _newtrack_0) false false))))))
    (:`then_2`
      (set `self.TimeUntilNextHeightCalc` (`KismetMathLibrary.RandomFloatInRange` 7.0 15.0) :!label _label_5)
      (`KismetSystemLibrary.Delay` (`self.TimeUntilNextHeightCalc`))
      (`KismetSystemLibrary.DelayUntilNextTick`)
      (`|ExecutionSequence`
        (:`then_0`
          (goto _label_3))
        (:`then_1`
          (goto _label_5))))
    (:`then_3`
      ;[1 1 1] Random Roaming
      (`|AIMoveTo` self (`NavigationSystemV1.K2_GetRandomReachablePointInRadius` (`self.K2_GetActorLocation`) 5000.0 null null) null 50.0 :!label _label_6
        (:`OnSuccess`
          _)
        (:`OnFail`
          _))
      (`KismetSystemLibrary.Delay` (`KismetMathLibrary.RandomFloatInRange` 2.0 5.0))
      (if (`self.Roaming`)
        (goto _label_6)))
    (:`then_4`
      ;[1 1 1] SaveMats
      (`|ExecutionSequence`
        (:`then_0`
          (bind _returnvalue (`PrimitiveComponent.CreateDynamicMaterialInstance` _ghostmesh 1 "/Game/CustomMaterials/Ghost_Mat.Ghost_Mat" "None"))
          (bind _output_get (set `self.GhostMat1` _returnvalue))
          (`PrimitiveComponent.SetMaterial` _ghostmesh_2 1 _output_get)
          (`MaterialInstanceDynamic.SetScalarParameterValue` _output_get "Transparency" 0.0)
          (`MaterialInstanceDynamic.SetScalarParameterValue` _output_get "TransparencyModifier" 0.0))
        (:`then_1`
          (bind _returnvalue_2 (`PrimitiveComponent.CreateDynamicMaterialInstance` _ghostmesh 3 "/Game/CustomMaterials/Ghost_Mat3.Ghost_Mat3" "None"))
          (bind _output_get_2 (set `self.GhostMat2` _returnvalue_2))
          (`PrimitiveComponent.SetMaterial` _ghostmesh_2 3 _output_get_2)
          (`MaterialInstanceDynamic.SetScalarParameterValue` _output_get_2 "Transparency" 0.0)
          (`MaterialInstanceDynamic.SetScalarParameterValue` _output_get_2 "TransparencyModifier" 0.0))
        (:`then_2`
          (bind _returnvalue_3 (`PrimitiveComponent.CreateDynamicMaterialInstance` _ghostmesh 4 "/Game/CustomMaterials/Ghost_Mat2.Ghost_Mat2" "None"))
          (bind _output_get_3 (set `self.GhostMat3` _returnvalue_3))
          (`PrimitiveComponent.SetMaterial` _ghostmesh_2 4 _output_get_3)
          (`MaterialInstanceDynamic.SetScalarParameterValue` _output_get_3 "Transparency" 0.0)
          (`MaterialInstanceDynamic.SetScalarParameterValue` _output_get_3 "TransparencyModifier" 0.0))
        (:`then_3`
          (bind _returnvalue_4 (`PrimitiveComponent.CreateDynamicMaterialInstance` _ghostmesh 2 "/Game/CustomMaterials/BlackCustomMat.BlackCustomMat" "None"))
          (bind _output_get_4 (set `self.GhostMat4` _returnvalue_4))
          (`PrimitiveComponent.SetMaterial` _ghostmesh_2 2 _output_get_4)
          (`MaterialInstanceDynamic.SetScalarParameterValue` _output_get_4 "Transparency" 0.0))))
    (:`then_5`)))

(event `RoamingFlying`
  ;[1 1 1] Control Roaming Flying
  (`|ExecutionSequence`
    (:`then_0`
      (goto _label_2))
    (:`then_1`
      (goto _label_5))))

(event `StopRoamingFlyingImmediately`
  ;[1 1 1] Control Roaming Flying
  (goto _label_4 :!via `Stop`))

(event `RandomRoam`
  ;[1 1 1] Random Roaming
  (goto _label_6))

(event `self.ReceiveAnyDamage`
  (params (Damage :type "Float (single-precision)") (DamageType :type "DamageType Object Reference") (InstigatedBy :type "Controller Object Reference") (DamageCauser :type "Actor Object Reference"))
  (bind (_returnvalue_roll _returnvalue_pitch _returnvalue_yaw) (`KismetMathLibrary.BreakRotator` (`KismetMathLibrary.MakeRotFromZ` (`KismetMathLibrary.GetDirectionUnitVector` (`self.K2_GetActorLocation` DamageCauser) (`self.K2_GetActorLocation`)))))
  ;[1 1 1] HandleDamage
  (if (not (`self.Dead`))
    (`/Engine/EditorBlueprintResources/StandardMacros.DoOnce` false
      (:`Completed`
        (`self.Death`)
        (`SceneComponent.K2_SetWorldRotation` (`self.GhostMesh`) (`KismetMathLibrary.MakeRotator` 0.0 0.0 _returnvalue_yaw) false false)))))

(event `Death`
  ;[1 1 1] handle death
  (set `SkeletalMeshComponent.GlobalAnimRateScale` (`KismetMathLibrary.RandomFloatInRange` 0.8 1.3) (`self.GhostMesh`))
  (set `self.Dead` true)
  (set `self.Roaming` false)
  (`NavMovementComponent.StopActiveMovement` (`self.CharacterMovement`))
  (`self.StopRoamingFlyingImmediately`)
  (`self.ShowGhost`))

(event `DeathExplosion`
  (bind _returnvalue (`KismetMathLibrary.RandomFloatInRange` 0.8 1.3))
  (bind _ghostmesh (`self.GhostMesh`))
  ;[1 1 1] HandleDeathExplosion
  (`/Engine/EditorBlueprintResources/StandardMacros.DoOnce` false
    (:`Completed`
      (`|ExecutionSequence`
        (:`then_0`
          (bind (_direction _newtrack_0) (`Timeline|Timeline` :!via `PlayFromStart`)
            (:`Update`
              (`SceneComponent.SetRelativeScale3D` _ghostmesh (`KismetMathLibrary.VLerp` (`SceneComponent.RelativeScale3D` _ghostmesh) (0.0 0.0 0.0) _newtrack_0)))))
        (:`then_1`
          (`KismetSystemLibrary.Delay` 0.6)
          (`GameplayStatics.SpawnEmitterAtLocation` "/Game/MarketplaceAssets/DreamscapeSeries/DreamscapeTower/Effects/P_GhostSparks.P_GhostSparks" (`SceneComponent.K2_GetComponentLocation` _ghostmesh) (`SceneComponent.K2_GetComponentRotation` _ghostmesh) (`KismetMathLibrary.MakeVector` _returnvalue _returnvalue _returnvalue))
          (`KismetSystemLibrary.Delay` 0.4)
          (`self.K2_DestroyActor`))))))

(event `self.ReceiveActorBeginOverlap`
  (params (OtherActor :type "Actor Object Reference"))
  (bind _capsule (`self.Capsule`))
  ;[1 1 1] HandleGhostVisibility
  (cast `/Game/Blueprints/Lighting/BP_FakeLanternLightDecal` OtherActor)
  (`self.ShowGhost`)
  (`|ExecutionSequence`
    (:`then_0`
      (if (not (`self.Visible`))
        (`/Engine/EditorBlueprintResources/StandardMacros.DoOnce` false
          (:`Completed`
            (`GameplayStatics.SpawnEmitterAtLocation` "/Game/MarketplaceAssets/DreamscapeSeries/DreamscapeTower/Effects/P_GhostSparks.P_GhostSparks" (`SceneComponent.K2_GetComponentLocation` _capsule) (`SceneComponent.K2_GetComponentRotation` _capsule) (0.3 0.3 0.3))))))))

(event `self.ReceiveActorEndOverlap`
  (params (OtherActor :type "Actor Object Reference"))
  ;[1 1 1] HandleGhostVisibility
  (cast `/Game/Blueprints/Lighting/BP_FakeLanternLightDecal` OtherActor)
  (`self.Hide Ghost`))

(event `ShowGhost`
  (bind _ghostmat1 (`self.GhostMat1`))
  (bind _ghostmat2 (`self.GhostMat2`))
  (bind _ghostmat3 (`self.GhostMat3`))
  ;[1 1 1] HandleGhostVisibility
  (`KismetSystemLibrary.DelayUntilNextTick`)
  (set `self.Visible` true)
  (bind (_direction _newtrack_0) (`Timeline|Fade` :!label _label_7)
    (:`Update`
      (`|ExecutionSequence`
        (:`then_0`
          (bind _returnvalue (`KismetMathLibrary.Lerp` 0.0 0.8 _newtrack_0))
          (`MaterialInstanceDynamic.SetScalarParameterValue` _ghostmat1 "Transparency" _returnvalue)
          (`MaterialInstanceDynamic.SetScalarParameterValue` _ghostmat1 "TransparencyModifier" _returnvalue))
        (:`then_1`
          (bind _returnvalue_2 (`KismetMathLibrary.Lerp` 0.0 0.9 _newtrack_0))
          (`MaterialInstanceDynamic.SetScalarParameterValue` _ghostmat2 "Transparency" _returnvalue_2)
          (`MaterialInstanceDynamic.SetScalarParameterValue` _ghostmat2 "TransparencyModifier" _returnvalue_2))
        (:`then_2`
          (bind _returnvalue_3 (`KismetMathLibrary.Lerp` 0.0 1.0 _newtrack_0))
          (`MaterialInstanceDynamic.SetScalarParameterValue` _ghostmat3 "Transparency" _returnvalue_3)
          (`MaterialInstanceDynamic.SetScalarParameterValue` _ghostmat3 "TransparencyModifier" _returnvalue_3))
        (:`then_3`
          (`MaterialInstanceDynamic.SetScalarParameterValue` (`self.GhostMat4`) "Transparency" _returnvalue_3))))))

(event `Hide Ghost`
  ;[1 1 1] HandleGhostVisibility
  (set `self.Visible` false)
  (goto _label_7 :!via `Reverse`))

(fn `UserConstructionScript`)