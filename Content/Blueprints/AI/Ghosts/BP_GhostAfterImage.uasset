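; BP_GhostAfterImage is a short-lived afterimage actor, apparently for ghost AI, that fades out and destroys itself.
; On BeginPlay it adds a skeletal mesh with paused animation at a given transform and gives each material slot a dynamic instance.
; A timeline, restarted inside that loop, lowers two transparency parameters to zero on the last-created instance, then destroys the actor.
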(event `self.ReceiveBeginPlay`
  (bind _returnvalue (`AddComponent|NODE_AddSkeletalMeshComponent-0`))
  (set `SkeletalMeshComponent.bPauseAnims` true _returnvalue)
  (`SceneComponent.K2_SetWorldTransform` _returnvalue (`self.New Transform`) false false)
  (for (_array_element _array_index) (`MeshComponent.GetMaterials` _returnvalue)
    (bind _returnvalue_2 (`KismetMaterialLibrary.CreateDynamicMaterialInstance` _array_element))
    (`PrimitiveComponent.SetMaterial` _returnvalue _array_index _returnvalue_2)
    (bind (_direction _newtrack_0) (`Timeline|Timeline` :!via `PlayFromStart`)
      (:`Update`
        (bind _returnvalue_3 (`KismetMathLibrary.Lerp` 0.5 0.0 _newtrack_0))
        (`MaterialInstanceDynamic.SetScalarParameterValue` _returnvalue_2 "Transparency" _returnvalue_3)
        (`MaterialInstanceDynamic.SetScalarParameterValue` _returnvalue_2 "TransparencyModifier" _returnvalue_3))
      (:`Finished`
        (`self.K2_DestroyActor`)))))

(fn `UserConstructionScript`)