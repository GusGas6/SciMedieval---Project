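; Crossbow bolt projectile with optional explosive and ice or lightning variants, which select its trail effect.
; On hit it damages anything except FirstPersonCharacter and sticks to the struck component on pawns.
; Explosive bolts detonate after a delay into an AoE bubble, trace down for a scorch decal, then destroy themselves.
; Lightning bolts repeatedly spawn small damage bubbles through a delay loop; ice bolts leave frozen ground on static mesh actors.
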(event `self.ReceiveBeginPlay`
  (bind _crossbowdamagetype (`self.CrossbowDamageType`))
  (bind _crossbowdamagetype_2 (`self.CrossbowDamageType`))
  (bind _trail (`self.trail`))
  (if (`self.Explosive`)
    (if (== _crossbowdamagetype_2 "/Game/Blueprints/HeathNDamage/DamageType_Ice.DamageType_Ice_C")
      (set `self.AoEDamageType` _crossbowdamagetype_2)
      (`NiagaraComponent.SetAsset` _trail "/Game/VFX/MarketplaceAssets/sA_Megapack_v1/sA_StylizedAttacksPack/FX/NiagaraSystems/NS_CartoonyFlameTrailIce.NS_CartoonyFlameTrailIce" true)
      (else
        (if (== _crossbowdamagetype_2 "/Game/Blueprints/HeathNDamage/DamageType_Lightning.DamageType_Lightning_C")
          (set `self.AoEDamageType` _crossbowdamagetype_2)
          (`NiagaraComponent.SetAsset` (`self.trail`) "/Game/VFX/MarketplaceAssets/sA_Megapack_v1/sA_StylizedAttacksPack/FX/NiagaraSystems/NS_CartoonyFlameTrailLightning.NS_CartoonyFlameTrailLightning" true)
          (`ActorComponent.Activate` (`self.Lightning`) true)
          (else
            (`NiagaraComponent.SetAsset` _trail "/Game/VFX/MarketplaceAssets/sA_Megapack_v1/sA_StylizedAttacksPack/FX/NiagaraSystems/NS_CartoonyFlameTrail.NS_CartoonyFlameTrail" true)))
        (`PrimitiveComponent.SetCollisionEnabled` (`self.Arrow`) "QueryAndPhysics")))
    (elif (== _crossbowdamagetype "/Game/Blueprints/HeathNDamage/DamageType_Ice.DamageType_Ice_C")
      (`NiagaraComponent.SetAsset` _trail "/Game/VFX/VFX/BP_RibbonArrowTrailFrost.BP_RibbonArrowTrailFrost" true)
      (elif (== _crossbowdamagetype "/Game/Blueprints/HeathNDamage/DamageType_Lightning.DamageType_Lightning_C")
        (`NiagaraComponent.SetAsset` _trail "/Game/VFX/VFX/BP_RibbonArrowTrailElectric.BP_RibbonArrowTrailElectric" true)
        (`ActorComponent.Activate` (`self.Lightning`) true)))))

(event `self.ReceiveHit`
  (params (MyComp :type "PrimitiveComponent Object Reference") (Other :type "Actor Object Reference") (OtherComp :type "PrimitiveComponent Object Reference") (bSelfMoved :type Boolean) (HitLocation :type "Vector Structure") (HitNormal :type "Vector Structure") (NormalImpulse :type "Vector Structure") (Hit :type "HitResult Structure (by ref)"))
  (bind _returnvalue (`SceneComponent.K2_GetComponentLocation` (`self.Arrow`)))
  (`|ExecutionSequence`
    (:`then_0`
      (cast `/Game/Blueprints/FirstPersonCharacter` Other
        (:`CastFailed`
          (`GameplayStatics.ApplyDamage` Other (* (`self.CrossbowBaseDamage`) 50.0) null (`GameplayStatics.GetPlayerPawn` 0) (`self.CrossbowDamageType`))
          (cast `Pawn` Other
            (:`then`
              (`|ExecutionSequence`
                (:`then_0`
                  (`SceneComponent.K2_AttachToComponent` (`self.Arrow`) OtherComp "None" "SnapToTarget" "KeepWorld" "KeepWorld" true)
                  (set `self.ArrowIsAttachToThis` OtherComp))))
            (:`CastFailed`
              _))
          (`PrimitiveComponent.SetCollisionEnabled` (`self.Sphere`) "NoCollision")
          (if (`self.Explosive`)
            (`|ExecutionSequence`
              (:`then_0`
                (`KismetSystemLibrary.Delay` 3.0)
                (`|SpawnActorFromClass` "/Game/Blueprints/HeathNDamage/BP_AoEBubble.BP_AoEBubble_C" (`KismetMathLibrary.MakeTransform` (`SceneComponent.K2_GetComponentLocation` (`self.Arrow`))) "Undefined" "MultiplyWithRoot" null 500.0 200.0 true false 600.0 (`self.AoEDamageType`) null)
                (bind (_outhit _returnvalue_2) (`KismetSystemLibrary.LineTraceSingleForObjects` _returnvalue (- _returnvalue (0.0 0.0 250.0)) (`|MakeArray` "ObjectTypeQuery1" :!type "EObjectTypeQuery Enum")))
                (if _returnvalue_2
                  (bind (_bblockinghit _binitialoverlap _time _distance _location _impactpoint _normal) (`GameplayStatics.BreakHitResult` _outhit))
                  (`|SpawnActorFromClass` "/Game/Blueprints/Lighting/BP_ScorchDecal.BP_ScorchDecal_C" (`KismetMathLibrary.MakeTransform` _location (`KismetMathLibrary.MakeRotFromZ` _normal) (2.0 2.0 2.0)) "AlwaysSpawn" "MultiplyWithRoot" null null))
                (`self.K2_DestroyActor`))
              (:`then_1`
                (if (== (`self.CrossbowDamageType`) "/Game/Blueprints/HeathNDamage/DamageType_Lightning.DamageType_Lightning_C") :!label _label
                  (`|SpawnActorFromClass` "/Game/Blueprints/HeathNDamage/BP_AoEBubble.BP_AoEBubble_C" (`KismetMathLibrary.MakeTransform` (`SceneComponent.K2_GetComponentLocation` (`self.Arrow`))) "Undefined" "MultiplyWithRoot" null 100.0 10.0 false false 0.0 "/Game/Blueprints/HeathNDamage/DamageType_Lightning.DamageType_Lightning_C" null :!label _label_2)
                  (`KismetSystemLibrary.Delay` 0.1)
                  (goto _label_2))))
            (else
              (`KismetSystemLibrary.Delay` 0.5)
              (`ActorComponent.Deactivate` (`self.trail`))
              (goto _label))))))
    (:`then_1`
      (if (== (`self.CrossbowDamageType`) "/Game/Blueprints/HeathNDamage/DamageType_Ice.DamageType_Ice_C")
        (cast `StaticMeshActor` Other)
        (`|SpawnActorFromClass` "/Game/Blueprints/MagicSpells/Ice/BP_FrozenGround.BP_FrozenGround_C" (`KismetMathLibrary.MakeTransform` HitLocation (`KismetMathLibrary.MakeRotFromZ` HitNormal) (0.2 0.2 0.2)) "Undefined" "MultiplyWithRoot" null null)))))

(fn `UserConstructionScript`)