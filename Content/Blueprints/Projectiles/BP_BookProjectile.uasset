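; Thrown book projectile that deals lightning damage, then returns to the player.
; Normally it detonates cannonballs and ricochets toward random nearby pawns, restarting its return timer on each bounce.
; In Tornado mode it stops and grows a vortex that repeatedly damages actors, applies impulses and launches the player.
; Returning, timed or forced, respawns the actor with return flags, homing to the player's sword mesh until ReturnBook fires on overlap.
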(event `self.ReceiveBeginPlay`
  (bind _array (`|MakeArray` "ObjectTypeQuery3" "ObjectTypeQuery8" "ObjectTypeQuery4" :!type "EObjectTypeQuery Enum"))
  (bind _projectilemovement (`self.ProjectileMovement`))
  (bind _bigtornado (`self.BigTornado`))
  (bind _tornadohurtcapsule (`self.TornadoHurtCapsule`))
  (bind _arrow (`self.Arrow`))
  (bind _projectilemovement_2 (`self.ProjectileMovement`))
  (bind _returnvalue (`SceneComponent.K2_GetComponentToWorld` _tornadohurtcapsule))
  (`|ExecutionSequence`
    (:`then_0`
      (`KismetSystemLibrary.Delay` 2.0 :!label _label)
      (`NiagaraComponent.ResetSystem` (`self.Niagara`))
      (goto _label))
    (:`then_1`
      (if (`self.Tornado`)
        (if (`self.ReturningToPlayer`)
          (`SceneComponent.SetVisibility` (`self.SmallDisk`) false false)
          (`SceneComponent.SetVisibility` (`self.BigTornado`) false false)
          (`PrimitiveComponent.SetCollisionEnabled` (`self.HurtBox`) "NoCollision")
          (`PrimitiveComponent.SetCollisionEnabled` (`self.TornadoHurtCapsule`) "NoCollision")
          (if (`self.ReturningToPlayer`) :!label _label_2
            (`PrimitiveComponent.SetCollisionResponseToAllChannels` (`self.Box`) "ECR_Overlap")
            (set `ProjectileMovementComponent.bIsHomingProjectile` true _projectilemovement_2)
            (bind _asfirst_person_character (cast `/Game/Blueprints/FirstPersonCharacter` (`GameplayStatics.GetPlayerCharacter` 0)))
            (set `ProjectileMovementComponent.HomingTargetComponent` (`/Game/Blueprints/FirstPersonCharacter.Mesh2PSword` _asfirst_person_character) _projectilemovement_2)
            (set `ProjectileMovementComponent.InitialSpeed` 10000.0 _projectilemovement_2)
            (set `ProjectileMovementComponent.MaxSpeed` 10000.0 _projectilemovement_2)
            (set `ProjectileMovementComponent.bRotationFollowsVelocity` true _projectilemovement_2)
            (set `MovementComponent.Velocity` (0.0 0.0 0.0) _projectilemovement_2)
            (bind (_direction _newtrack_0) (`Timeline|Timeline` :!via `PlayFromStart`)
              (:`Update`
                (set `ProjectileMovementComponent.HomingAccelerationMagnitude` (`KismetMathLibrary.Lerp` 0.0 9999999.0 _newtrack_0) _projectilemovement_2)))
            (else
              (if (`self.Tornado`) :!label _label_3
                (`|ExecutionSequence`
                  (:`then_0`
                    (`Timeline|Timeline_0` :!via `Stop` :!label _label_4
                      (:`Finished`
                        (`self.ReturnToPlayer`))))
                  (:`then_1`
                    (`KismetSystemLibrary.DelayUntilNextTick`)
                    (if (not (`self.ReturningToPlayer`))
                      (goto _label_4 :!via `PlayFromStart`))))
                (else
                  (`|ExecutionSequence`
                    (:`then_0`
                      (`Timeline|TimelineToReturn` :!via `Stop` :!label _label_5
                        (:`Finished`
                          (`self.ReturnToPlayer`))))
                    (:`then_1`
                      (`KismetSystemLibrary.DelayUntilNextTick`)
                      (if (`self.ReturningToPlayer`)
                        (`|SpawnActorFromClass` "BP_BookProjectile_C" (`self.GetTransform`) "Undefined" "MultiplyWithRoot" null 5.0 false (0.0 0.0 3000.0) (`self.Slicer`) (`self.Tornado`) false null)
                        (`self.K2_DestroyActor`)
                        (else
                          (goto _label_5 :!via `PlayFromStart`)))))))))
          (else
            (`SceneComponent.SetVisibility` _bigtornado true false)
            (`SceneComponent.SetVisibility` (`self.SmallDisk`) true false)
            (`|ExecutionSequence`
              (:`then_0`
                (set `MovementComponent.Velocity` (* (`MovementComponent.Velocity` _projectilemovement) 0.4) _projectilemovement)
                (`KismetSystemLibrary.Delay` 0.5)
                (set `MovementComponent.Velocity` (0.0 0.0 0.0) (`self.ProjectileMovement`))
                (`SceneComponent.SetVisibility` (`self.SmallDisk`) false false)
                (`SceneComponent.SetVisibility` (`self.Niagara`) false false)
                (`PrimitiveComponent.SetCollisionEnabled` (`self.HurtBox`) "NoCollision")
                (`PrimitiveComponent.SetCollisionEnabled` (`self.TornadoHurtCapsule`) "QueryAndPhysics")
                (`PrimitiveComponent.SetCollisionEnabled` (`self.SmallDisk`) "QueryAndPhysics")
                (goto _label_2))
              (:`then_1`
                (`KismetSystemLibrary.Delay` 0.3)
                (bind (_direction_2 _newtrack_0_2) (`Timeline|BigTornadoGrow` :!via `PlayFromStart`)
                  (:`Update`
                    (`SceneComponent.SetRelativeScale3D` _bigtornado (`KismetMathLibrary.VLerp` (0.0 0.0 0.0) (3.0 3.0 3.0) _newtrack_0_2)))))
              (:`then_2`
                (`KismetSystemLibrary.Delay` 0.001)
                (`|ExecutionSequence` :!label _label_6
                  (:`then_0`
                    (bind _outactors (`KismetSystemLibrary.ComponentOverlapActors` _tornadohurtcapsule _returnvalue _array))
                    (for _array_element _outactors
                      (bind _asfirst_person_character_2 (cast `/Game/Blueprints/FirstPersonCharacter` _array_element)
                        (:`then`
                          (`Character.LaunchCharacter` _asfirst_person_character_2 (* (`SceneComponent.GetForwardVector` _arrow) 599.0) false false))
                        (:`CastFailed`
                          (`GameplayStatics.ApplyDamage` _array_element (`self.BookDamage`) null self "/Game/Blueprints/HeathNDamage/DamageType_Lightning.DamageType_Lightning_C"))))
                    (`KismetSystemLibrary.Delay` 0.05)
                    (goto _label_6))
                  (:`then_1`
                    (bind _outcomponents (`KismetSystemLibrary.ComponentOverlapComponents` _tornadohurtcapsule _returnvalue _array :!label _label_7))
                    (for _array_element_2 _outcomponents
                      (`PhysicsObjectBlueprintLibrary.ApplyRadialImpulse` _array_element_2 (`SceneComponent.K2_GetComponentLocation` _arrow) 800.0 50000.0 "RIF_Constant"))
                    (`KismetSystemLibrary.Delay` 0.05)
                    (goto _label_7)))))))
        (else
          (`SceneComponent.SetVisibility` (`self.SmallDisk`) true false)
          (`SceneComponent.SetVisibility` (`self.Niagara`) true false)
          (`SceneComponent.SetVisibility` (`self.BigTornado`) false false)
          (`PrimitiveComponent.SetCollisionEnabled` (`self.HurtBox`) "QueryAndPhysics")
          (`PrimitiveComponent.SetCollisionEnabled` (`self.TornadoHurtCapsule`) "NoCollision")
          (goto _label_2))))))

(event `self.ReturnToPlayerCapsule.OnComponentBeginOverlap`
  (params (OverlappedComponent :type "PrimitiveComponent Object Reference") (OtherActor :type "Actor Object Reference") (OtherComp :type "PrimitiveComponent Object Reference") (OtherBodyIndex :type Integer) (bFromSweep :type Boolean) (SweepResult :type "HitResult Structure (by ref)"))
  (bind _asfirst_person_character (cast `/Game/Blueprints/FirstPersonCharacter` OtherActor))
  (if (`self.ReturningToPlayer`)
    (`/Engine/EditorBlueprintResources/StandardMacros.DoOnce` false
      (:`Completed`
        (`/Game/Blueprints/FirstPersonCharacter.ReturnBook` _asfirst_person_character)
        (`self.K2_DestroyActor`)))))

(event `self.HurtBox.OnComponentBeginOverlap`
  (params (OverlappedComponent :type "PrimitiveComponent Object Reference") (OtherActor :type "Actor Object Reference") (OtherComp :type "PrimitiveComponent Object Reference") (OtherBodyIndex :type Integer) (bFromSweep :type Boolean) (SweepResult :type "HitResult Structure (by ref)"))
  (if (not (`self.Tornado`))
    (bind _asbp_cannonball (cast `/Game/Blueprints/Interactibles/BP_Cannonball` OtherActor)
      (:`then`
        (`/Game/Blueprints/Interactibles/BP_Cannonball.Explode` _asbp_cannonball))
      (:`CastFailed`
        _))
    (cast `/Game/Blueprints/FirstPersonCharacter` OtherActor
      (:`CastFailed`
        (`GameplayStatics.ApplyDamage` OtherActor (`self.BookDamage`) null self "/Game/Blueprints/HeathNDamage/DamageType_Lightning.DamageType_Lightning_C")
        (if (not (`self.ForcingReturn`))
          (set `self.SpeedAfterHit` (* (`self.SpeedAfterHit`) 1.0))
          (bind (_outactors _returnvalue) (`KismetSystemLibrary.SphereOverlapActors` (`self.K2_GetActorLocation`) 3000.0 (`|MakeArray` "ObjectTypeQuery3" :!type "EObjectTypeQuery Enum") null (`|MakeArray` (`GameplayStatics.GetPlayerCharacter` 0) :!type "Actor Object Reference")))
          (if _returnvalue
            (`|ExecutionSequence`
              (:`then_0`
                (goto _label_3))
              (:`then_1`
                (set `MovementComponent.Velocity` (* (`KismetMathLibrary.GetDirectionUnitVector` (`self.K2_GetActorLocation`) (`self.K2_GetActorLocation` (`KismetArrayLibrary.Array_Random` _outactors))) (`self.SpeedAfterHit`)) (`self.ProjectileMovement`))))))
        (bind _asbp_target_dummy (cast `/Game/Blueprints/AI/BP_TargetDummy` OtherActor))))))

(event `ReturnToPlayer`
  (`|SpawnActorFromClass` "BP_BookProjectile_C" (`self.GetTransform`) "AlwaysSpawn" "MultiplyWithRoot" null 5.0 true (0.0 0.0 3000.0) (`self.Slicer`) (`self.Tornado`) false null)
  (`self.K2_DestroyActor`))

(event `ForceReturnToPlayer`
  (`|SpawnActorFromClass` "BP_BookProjectile_C" (`self.GetTransform`) "AlwaysSpawn" "MultiplyWithRoot" null 5.0 true (0.0 0.0 3000.0) (`self.Slicer`) (`self.Tornado`) true null)
  (`self.K2_DestroyActor`))

(fn `UserConstructionScript`)