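; Test damage projectile that the player can parry or block, with optional homing on the player that stops at close range.
; Overlapping during parry or kick-parry frames reverses and speeds it up, ends homing and triggers the player's SpellParry.
; Hits send a shield-breaking HitBlock when blocked, otherwise apply damage (pierce type for non-players), then explode and destroy it.
; The Parried start-up boost serves an older respawn-based parry, now disconnected.
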(event `self.ReceiveBeginPlay`
  (bind _projectilemovement (`self.ProjectileMovement`))
  (bind _projectilemovement_2 (`self.ProjectileMovement`))
  (`|ExecutionSequence`
    (:`then_0`
      (if (`self.Parried`)
        (set `ProjectileMovementComponent.MaxSpeed` (* (`MovementComponent.GetMaxSpeed` _projectilemovement) 3.0) _projectilemovement)
        (`KismetSystemLibrary.DelayUntilNextTick`)
        (set `MovementComponent.Velocity` (* (`MovementComponent.Velocity` _projectilemovement) 3.0) _projectilemovement)
        (`PrimitiveComponent.SetCollisionResponseToChannel` (`self.Sphere1`) "ECC_GameTraceChannel2" "ECR_Ignore")))
    (:`then_1`
      (if (`self.Homing`)
        (set `ProjectileMovementComponent.bIsHomingProjectile` true _projectilemovement_2)
        (bind _asbp_third_person_character (cast `/Game/Blueprints/BP_ThirdPersonCharacter` (`GameplayStatics.GetPlayerCharacter` 0)))
        (set `ProjectileMovementComponent.HomingTargetComponent` (`/Game/Blueprints/BP_ThirdPersonCharacter.Capsule` _asbp_third_person_character) _projectilemovement_2)
        (if (<= (`KismetMathLibrary.VSize` (- (`self.K2_GetActorLocation` _asbp_third_person_character) (`self.K2_GetActorLocation`))) 100.0) :!label _label
          (set `ProjectileMovementComponent.bIsHomingProjectile` false (`self.ProjectileMovement`))
          (else
            (`KismetSystemLibrary.DelayUntilNextTick`)
            (goto _label)))))))

(event `self.ReceiveActorBeginOverlap`
  (params (OtherActor :type "Actor Object Reference"))
  (bind _sphere1 (`self.Sphere1`))
  (bind _projectilemovement (`self.ProjectileMovement`))
  (bind _asbp_third_person_character (cast `/Game/Blueprints/BP_ThirdPersonCharacter` OtherActor))
  (if (or (`/Game/Blueprints/BP_ThirdPersonCharacter.KickParryFramesActive` _asbp_third_person_character) (`/Game/Blueprints/BP_ThirdPersonCharacter.ParryFramesActive` _asbp_third_person_character))
    (`/Engine/EditorBlueprintResources/StandardMacros.DoOnce` false
      (:`Completed`
        (set `MovementComponent.Velocity` (* (`MovementComponent.Velocity` _projectilemovement) -2.0) _projectilemovement)
        (set `ProjectileMovementComponent.MaxSpeed` (* (`MovementComponent.GetMaxSpeed` _projectilemovement) 2.0) _projectilemovement)
        (set `ProjectileMovementComponent.bIsHomingProjectile` false _projectilemovement)
        (`/Game/Blueprints/BP_ThirdPersonCharacter.SpellParry` _asbp_third_person_character (`SceneComponent.K2_GetComponentLocation` _sphere1) (`SceneComponent.K2_GetComponentRotation` _sphere1))))))

(event `self.ReceiveHit`
  (params (MyComp :type "PrimitiveComponent Object Reference") (Other :type "Actor Object Reference") (OtherComp :type "PrimitiveComponent Object Reference") (bSelfMoved :type Boolean) (HitLocation :type "Vector Structure") (HitNormal :type "Vector Structure") (NormalImpulse :type "Vector Structure") (Hit :type "HitResult Structure (by ref)"))
  (bind _asbp_third_person_character (cast `/Game/Blueprints/BP_ThirdPersonCharacter` Other)
    (:`then`
      (`/Engine/EditorBlueprintResources/StandardMacros.DoOnce` false
        (:`Completed`
          (`KismetSystemLibrary.PrintString` (`KismetSystemLibrary.GetDisplayName` OtherComp))
          (bind _returnvalue (== OtherComp (`/Game/Blueprints/BP_ThirdPersonCharacter.BlockBox` _asbp_third_person_character)))
          (if (and (`/Game/Blueprints/BP_ThirdPersonCharacter.ParryFramesActive` _asbp_third_person_character) _returnvalue)
            _
            (elif (and (== OtherComp (`/Game/Blueprints/BP_ThirdPersonCharacter.KickParryBox` _asbp_third_person_character)) (`/Game/Blueprints/BP_ThirdPersonCharacter.KickParryFramesActive` _asbp_third_person_character))
              _
              (else
                _)))
          (if (and _returnvalue (`/Game/Blueprints/BP_ThirdPersonCharacter.Blocking` _asbp_third_person_character))
            (`/Game/Blueprints/BP_ThirdPersonCharacter.HitBlock` _asbp_third_person_character (`self.K2_GetActorLocation`) (`self.Damage`) true)
            (else
              (`GameplayStatics.ApplyDamage` _asbp_third_person_character (`self.Damage`) null self))))))
    (:`CastFailed`
      (`GameplayStatics.ApplyDamage` Other (`self.Damage`) null self "/Game/Blueprints/HeathNDamage/DamageType_Pierce.DamageType_Pierce_C")))
  (`GameplayStatics.SpawnEmitterAtLocation` "/Game/StarterContent/Particles/P_Explosion.P_Explosion" (`self.K2_GetActorLocation`) (struct) (0.3 0.3 0.3))
  (`self.K2_DestroyActor`))

(fn `UserConstructionScript`)