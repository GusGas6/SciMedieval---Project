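; Thrown sword projectile that damages what it overlaps, spraying blood on target dummies, and returns to the first-person player.
; After a short delay it replaces itself with a returning copy that overlaps everything and homes on the player's sword mesh with timeline-ramped acceleration.
; Hitting a surface beforehand swaps it for a sword-in-ground actor.
; When the returning copy reaches the player, it clears the thrown state, restores sword handling and destroys itself.
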(event `self.ReceiveBeginPlay`
  (bind _projectilemovement (`self.ProjectileMovement`))
  (if (`self.ReturningToPlayer`)
    (`PrimitiveComponent.SetCollisionResponseToAllChannels` (`self.Box`) "ECR_Overlap")
    (set `ProjectileMovementComponent.bIsHomingProjectile` true _projectilemovement)
    (bind _asfirst_person_character (cast `/Game/Blueprints/FirstPersonCharacter` (`GameplayStatics.GetPlayerCharacter` 0)))
    (set `ProjectileMovementComponent.HomingTargetComponent` (`/Game/Blueprints/FirstPersonCharacter.Mesh2PSword` _asfirst_person_character) _projectilemovement)
    (set `ProjectileMovementComponent.InitialSpeed` 10000.0 _projectilemovement)
    (set `ProjectileMovementComponent.MaxSpeed` 10000.0 _projectilemovement)
    (set `ProjectileMovementComponent.bRotationFollowsVelocity` true _projectilemovement)
    (set `MovementComponent.Velocity` (0.0 0.0 1200.0) _projectilemovement)
    (bind (_direction _newtrack_0) (`Timeline|Timeline` :!via `PlayFromStart`)
      (:`Update`
        (set `ProjectileMovementComponent.HomingAccelerationMagnitude` (`KismetMathLibrary.Lerp` 0.0 9999999.0 _newtrack_0) _projectilemovement)))
    (else
      (`KismetSystemLibrary.Delay` 0.75)
      (`self.ReturnToPlayer`))))

(event `self.ReturnToPlayerCapsule.OnComponentBeginOverlap`
  (params (OverlappedComponent :type "PrimitiveComponent Object Reference") (OtherActor :type "Actor Object Reference") (OtherComp :type "PrimitiveComponent Object Reference") (OtherBodyIndex :type Integer) (bFromSweep :type Boolean) (SweepResult :type "HitResult Structure (by ref)"))
  (bind _asfirst_person_character (cast `/Game/Blueprints/FirstPersonCharacter` OtherActor))
  (if (`self.ReturningToPlayer`)
    (`/Engine/EditorBlueprintResources/StandardMacros.DoOnce` false
      (:`Completed`
        (set `/Game/Blueprints/FirstPersonCharacter.SwordThrown` false _asfirst_person_character)
        (if (not (`/Game/Blueprints/FirstPersonCharacter.GunEquipped` _asfirst_person_character))
          (if (not (`/Game/Blueprints/FirstPersonCharacter.StaffEquipped` _asfirst_person_character))
            (`/Game/Blueprints/FirstPersonCharacter.ForceEquipSword` _asfirst_person_character))
          (`/Game/Blueprints/FirstPersonCharacter.StopGunSpinning` _asfirst_person_character))
        (`/Game/Blueprints/FirstPersonCharacter.SwordReturned` _asfirst_person_character)
        (`self.K2_DestroyActor`)))))

(event `self.HurtBox.OnComponentBeginOverlap`
  (params (OverlappedComponent :type "PrimitiveComponent Object Reference") (OtherActor :type "Actor Object Reference") (OtherComp :type "PrimitiveComponent Object Reference") (OtherBodyIndex :type Integer) (bFromSweep :type Boolean) (SweepResult :type "HitResult Structure (by ref)"))
  (cast `/Game/Blueprints/FirstPersonCharacter` OtherActor
    (:`CastFailed`
      (`GameplayStatics.ApplyDamage` OtherActor (`self.ThrownSwordDamage`) null self)
      (bind _asbp_target_dummy (cast `/Game/Blueprints/AI/BP_TargetDummy` OtherActor))
      (for _ (range 6)
        (bind _returnvalue (`SceneComponent.GetSocketLocation` (`/Game/Blueprints/AI/BP_TargetDummy.SkeletalMesh` _asbp_target_dummy) "Spine"))
        (bind _returnvalue_2 (`KismetMathLibrary.MakeRotFromZ` (`KismetMathLibrary.RandomUnitVectorInConeInDegrees` (`KismetMathLibrary.GetDirectionUnitVector` (`SceneComponent.K2_GetComponentLocation` (`self.Box`)) _returnvalue) 10.0)))
        (`GameplayStatics.SpawnEmitterAttached` "/Game/MarketplaceAssets/Realistic_Starter_VFX_Pack_Vol2/Particles/Blood/P_Blood_Splat_Cone.P_Blood_Splat_Cone" (`.HitComponent` (`GameplayStatics.BreakHitResult` SweepResult)) "None" _returnvalue _returnvalue_2 (1.5 1.5 1.5) "KeepWorldPosition")
        (`GameplayStatics.SpawnEmitterAtLocation` "/Game/VFX/Bonuses/P_BulletImpact_Meat.P_BulletImpact_Meat" _returnvalue _returnvalue_2 (0.1 0.1 0.1))))))

(event `ReturnToPlayer`
  (`|SpawnActorFromClass` "BP_SwordProjectile_C" (`self.GetTransform`) "AlwaysSpawn" "MultiplyWithRoot" null 100.0 true (0.0 0.0 3000.0) null)
  (`self.K2_DestroyActor`))

(event `self.ReceiveHit`
  (params (MyComp :type "PrimitiveComponent Object Reference") (Other :type "Actor Object Reference") (OtherComp :type "PrimitiveComponent Object Reference") (bSelfMoved :type Boolean) (HitLocation :type "Vector Structure") (HitNormal :type "Vector Structure") (NormalImpulse :type "Vector Structure") (Hit :type "HitResult Structure (by ref)"))
  (bind (_returnvalue_location _returnvalue_rotation _returnvalue_scale) (`KismetMathLibrary.BreakTransform` (`self.GetTransform`)))
  (`|SpawnActorFromClass` "/Game/Blueprints/Unique/BP_SwordInGroundActor.BP_SwordInGroundActor_C" (`KismetMathLibrary.MakeTransform` _returnvalue_location _returnvalue_rotation _returnvalue_scale) "Undefined" "MultiplyWithRoot" null (`self.Launch Velocity`) (`KismetMathLibrary.MakeRotFromZ` HitNormal) null)
  (`GameplayStatics.SpawnEmitterAtLocation` "/Game/VFX/Bonuses/P_BulletImpact.P_BulletImpact" HitLocation (`KismetMathLibrary.MakeRotFromZ` HitNormal) (0.5 0.5 0.5))
  (`self.K2_DestroyActor`))

(fn `UserConstructionScript`)