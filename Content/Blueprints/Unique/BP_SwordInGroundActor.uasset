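; Player's sword left stuck in the ground, which can fly back to the player as a BP_SwordProjectile.
; BeginPlay orients the light and, for overhead throws, the mesh, then briefly delays enabling collision and showing the light.
; ReturnToPlayer or DamageType_ReturnToPlayer damage replaces the actor with a returning projectile; the damage path also transfers the mesh.
; Player overlap while HookedIntoAnchor triggers instant collection.
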(event `self.ReceiveBeginPlay`
  (bind _fakelight (`self.FakeLight`))
  (`SceneComponent.K2_SetWorldRotation` (`self.FakeLight`) (`self.FakeBlueLightRotation`) false false)
  (`|ExecutionSequence`
    (:`then_0`
      (if (`self.Overhead`)
        (`SceneComponent.K2_SetRelativeRotation` (`self.Greatsword`) (`self.Greathammer Rotation`) false false)))
    (:`then_1`
      (`KismetSystemLibrary.Delay` 0.02)
      (`PrimitiveComponent.SetCollisionEnabled` (`self.Box`) "QueryAndPhysics")
      (`/Engine/EditorBlueprintResources/StandardMacros.IsValid` _fakelight
        (:`Is Valid`
          (`SceneComponent.SetVisibility` _fakelight true false))))))

(event `self.ReceiveActorBeginOverlap`
  (params (OtherActor :type "Actor Object Reference"))
  ;[1 0.572 0] unhooked due to weapon meshes
  (if (`self.HookedIntoAnchor`)
    (bind _asfirst_person_character (cast `/Game/Blueprints/FirstPersonCharacter` OtherActor))
    (`/Game/Blueprints/FirstPersonCharacter.ToggleInstantSwordCollection` _asfirst_person_character (`StaticMeshComponent.StaticMesh` (`self.Greatsword`)))
    (`self.K2_DestroyActor`)))

(event `ReturnToPlayer`
  (bind _returnvalue (`self.GetTransform`))
  (bind _greathammer_rotation (`self.Greathammer Rotation`))
  (if (`self.Overhead`)
    (`|SpawnActorFromClass` "/Game/Blueprints/Projectiles/BP_SwordProjectile.BP_SwordProjectile_C" (`KismetMathLibrary.MakeTransform` (.location _returnvalue) (`KismetMathLibrary.MakeRotator` (+ (.roll (.rotation _returnvalue)) -90.0) (.pitch (.rotation _returnvalue)) (.yaw (.rotation _returnvalue))) (.scale _returnvalue)) "AlwaysSpawn" "MultiplyWithRoot" null 0.1 true (0.0 0.0 3000.0) false false false false (struct) _greathammer_rotation true (10000.0 10000.0 0.0) false null)
    (else
      (`|SpawnActorFromClass` "/Game/Blueprints/Projectiles/BP_SwordProjectile.BP_SwordProjectile_C" (`self.GetTransform`) "AlwaysSpawn" "MultiplyWithRoot" null 0.1 true (0.0 0.0 3000.0) false false false false (struct) _greathammer_rotation true (10000.0 10000.0 0.0) false null)))
  (`self.K2_DestroyActor`))

(event `self.ReceiveAnyDamage`
  (params (Damage :type "Float (single-precision)") (DamageType :type "DamageType Object Reference") (InstigatedBy :type "Controller Object Reference") (DamageCauser :type "Actor Object Reference"))
  (bind _returnvalue (`SceneComponent.K2_GetComponentToWorld` (`self.Greatsword`)))
  (bind _staticmesh (`StaticMeshComponent.StaticMesh` (`self.Greatsword`)))
  ;[1 0 0.5809] TODO: MAKE THIS WORK WITH IN GROUND ACTORS
  (if (== (`GameplayStatics.GetObjectClass` DamageType) "/Game/Blueprints/HeathNDamage/DamageType_ReturnToPlayer.DamageType_ReturnToPlayer_C")
    (bind _asfirst_person_character (cast `/Game/Blueprints/FirstPersonCharacter` (`GameplayStatics.GetPlayerCharacter` 0)))
    (set `/Game/Blueprints/FirstPersonCharacter.WeaponIsReturning` true _asfirst_person_character)
    (bind _returnvalue_2 (`|SpawnActorFromClass` "/Game/Blueprints/Projectiles/BP_SwordProjectile.BP_SwordProjectile_C" _returnvalue "AlwaysSpawn" "MultiplyWithRoot" null 0.1 true (0.0 0.0 3000.0) false false false false (struct) (struct :`Pitch` -90.0 :`Yaw` 720.000927 :`Roll` 1079.99907) true (10000.0 10000.0 0.0) false null))
    (bind _greatsword (`/Game/Blueprints/Projectiles/BP_SwordProjectile.Greatsword` _returnvalue_2))
    (`SceneComponent.K2_SetWorldTransform` _greatsword _returnvalue false false)
    (if (== _staticmesh "/Game/Blueprints/Interactibles/BP_EnemySwordPhysicsObject.BP_EnemySwordPhysicsObject")
      (`StaticMeshComponent.SetStaticMesh` _greatsword "/Game/Models/Weapons/SM_Sword1.SM_Sword1")
      (`self.K2_DestroyActor`)
      (else
        (`StaticMeshComponent.SetStaticMesh` _greatsword _staticmesh)
        (`self.K2_DestroyActor`)))))

(fn `UserConstructionScript`)