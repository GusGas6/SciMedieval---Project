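; BP_AoEBubble is a short-lived area-of-effect actor that damages what overlaps its radius-sized sphere, then destroys itself.
; In explosion mode, BeginPlay spawns radius-scaled explosive, ice or lightning effects plus a BP_ForceActor for knockback.
; Overlapped characters blocking toward the blast take a shield-breaking HitBlock; others take typed damage and a launch scaled by damage.
; Outside explosion mode, it only damages third-person characters with capsule collision enabled.
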(event `self.ReceiveBeginPlay`
  (bind _returnvalue (`self.K2_GetActorLocation`))
  (bind _returnvalue_2 (`self.K2_GetActorRotation`))
  (bind _explosiondamagetype (`self.ExplosionDamageType`))
  (bind _returnvalue_3 (* (/ (`self.AreaOfEffectRadius`) 250.0) (1.0 1.0 1.0)))
  (`SphereComponent.SetSphereRadius` (`self.AreaOfEffectSphere`) (`self.AreaOfEffectRadius`) true)
  (`|ExecutionSequence`
    (:`then_0`
      (`KismetSystemLibrary.Delay` 0.2)
      (`self.K2_DestroyActor`))
    (:`then_1`
      (if (`self.Explosion?`)
        (if (== _explosiondamagetype "/Game/Blueprints/HeathNDamage/DamageType_Explosive.DamageType_Explosive_C")
          (`NiagaraFunctionLibrary.SpawnSystemAtLocation` "/Game/VFX/Bonuses/P_Poof_Yellow.P_Poof_Yellow" _returnvalue _returnvalue_2 _returnvalue_3)
          (`GameplayStatics.SpawnEmitterAtLocation` "/Game/VFX/Bonuses/P_Explosion_No_Smoke.P_Explosion_No_Smoke" _returnvalue _returnvalue_2 _returnvalue_3)
          (`GameplayStatics.SpawnEmitterAtLocation` "/Game/VFX/InfinityBladeEffects/Effects/FX_Breakables/barrel/BP_ExplosiveBarrelBreakable.BP_ExplosiveBarrelBreakable" _returnvalue _returnvalue_2 (2.0 2.0 2.0))
          (`|SpawnActorFromClass` "/Game/Blueprints/Interactibles/BP_ForceActor.BP_ForceActor_C" (`KismetMathLibrary.MakeTransform` (`self.K2_GetActorLocation`)) "Undefined" "MultiplyWithRoot" null true (`self.ExplosionKnockbackForce`) (`self.AreaOfEffectRadius`) (`self.ShowDebugSphere`) null :!label _label)
          (elif (== _explosiondamagetype "/Game/Blueprints/HeathNDamage/DamageType_Ice.DamageType_Ice_C")
            (`GameplayStatics.SpawnEmitterAtLocation` "/Game/MarketplaceAssets/FXVarietyPack/Particles/Frost_AoE_Blast.Frost_AoE_Blast" _returnvalue _returnvalue_2 _returnvalue_3)
            (`NiagaraFunctionLibrary.SpawnSystemAtLocation` "/Game/VFX/Bonuses/P_Poof_Ice.P_Poof_Ice" _returnvalue _returnvalue_2 _returnvalue_3)
            (`GameplayStatics.SpawnEmitterAtLocation` "/Game/VFX/Bonuses/P_Explosion_No_Smoke.P_Explosion_No_Smoke" _returnvalue _returnvalue_2 _returnvalue_3)
            (goto _label)
            (elif (== _explosiondamagetype "/Game/Blueprints/HeathNDamage/DamageType_Lightning.DamageType_Lightning_C")
              (`GameplayStatics.SpawnEmitterAtLocation` "/Game/MarketplaceAssets/FXVarietyPack/Particles/P_ky_lightning3.P_ky_lightning3" _returnvalue _returnvalue_2 _returnvalue_3)
              (`GameplayStatics.SpawnEmitterAtLocation` "/Game/VFX/Bonuses/P_Explosion_No_Smoke.P_Explosion_No_Smoke" _returnvalue _returnvalue_2 _returnvalue_3)
              (goto _label))))))
    (:`then_2`
      (if (`self.ShowDebugSphere`)
        (`SceneComponent.SetVisibility` (`self.AreaOfEffectSphere`) true false)))))

(event `self.ReceiveActorBeginOverlap`
  (params (OtherActor :type "Actor Object Reference"))
  (bind _explosiondamagetype (`self.ExplosionDamageType`))
  (bind _aoedamage (`self.AoEDamage`))
  (if (`self.Explosion?`)
    (bind _asbp_third_person_character (cast `/Game/Blueprints/BP_ThirdPersonCharacter` OtherActor)
      (:`then`
        (if (not (== (`PrimitiveComponent.GetCollisionEnabled` (`/Game/Blueprints/BP_ThirdPersonCharacter.Capsule` _asbp_third_person_character)) 0))
          (bind _returnvalue (`KismetMathLibrary.DegAcos` (`KismetMathLibrary.Dot_VectorVector` (`KismetMathLibrary.Normal` (- (`self.K2_GetActorLocation`) (`self.K2_GetActorLocation` _asbp_third_person_character))) (`self.GetActorForwardVector` _asbp_third_person_character))))
          (if (and (<= _returnvalue 70.0) (>= _returnvalue -70.0) (`/Game/Blueprints/BP_ThirdPersonCharacter.Blocking` _asbp_third_person_character))
            (`/Game/Blueprints/BP_ThirdPersonCharacter.HitBlock` _asbp_third_person_character (`self.K2_GetActorLocation`) _aoedamage true)
            (else
              (`GameplayStatics.ApplyDamage` OtherActor _aoedamage null self _explosiondamagetype :!label _label_2)
              (bind _asbp_third_person_character_2 (cast `/Game/Blueprints/BP_ThirdPersonCharacter` OtherActor))
              (bind _returnvalue_2 (* (`KismetMathLibrary.GetDirectionUnitVector` (`self.K2_GetActorLocation`) (`self.K2_GetActorLocation` _asbp_third_person_character_2)) (`self.AoEDamage`) 20.0))
              (`Character.LaunchCharacter` _asbp_third_person_character_2 _returnvalue_2 false false)
              (`KismetSystemLibrary.PrintString` (`KismetStringLibrary.Conv_VectorToString` _returnvalue_2))))))
      (:`CastFailed`
        (goto _label_2)))
    (else
      (bind _asbp_third_person_character_3 (cast `/Game/Blueprints/BP_ThirdPersonCharacter` OtherActor))
      (if (not (== (`PrimitiveComponent.GetCollisionEnabled` (`/Game/Blueprints/BP_ThirdPersonCharacter.Capsule` _asbp_third_person_character_3)) 0))
        (`GameplayStatics.ApplyDamage` OtherActor _aoedamage null self _explosiondamagetype)))))

(fn `UserConstructionScript`)