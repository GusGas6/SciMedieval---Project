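; Base gib actor for AI: a physics mesh that spurts blood, then scales by timeline and destroys itself after about a minute.
; Randomly timed spurts impulse the mesh, slowing once no longer freshly gibbed; frozen gibs get ice material and stop spurting.
; Fast-moving gibs damage pawns by velocity and bounce back, adding lightning damage while electrified.
; Incoming damage pushes it radially, temporarily electrifies it, or turns it into a sword projectile returning to the player.
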(event `self.ReceiveBeginPlay`
  (bind _staticmesh (`self.StaticMesh`))
  (bind _staticmesh_2 (`self.StaticMesh`))
  (`|ExecutionSequence`
    (:`then_0`
      (`KismetSystemLibrary.Delay` (`KismetMathLibrary.RandomFloatInRange` 1.5 4.0))
      (set `self.RecentlyGibbed` false)
      (`KismetSystemLibrary.Delay` 50.0)
      (bind (_direction _newtrack_0) (`Timeline|Timeline` :!via `PlayFromStart`)
        (:`Update`
          (`self.SetActorScale3D` (`KismetMathLibrary.VLerp` (0.0 0.0 0.0) (1.0 1.0 1.0) _newtrack_0)))
        (:`Finished`
          (`self.K2_DestroyActor`))))
    (:`then_1`
      (`KismetSystemLibrary.Delay` (`KismetMathLibrary.RandomFloatInRange` 0.2 0.6) :!label _label)
      (bind _returnvalue (`GameplayStatics.SpawnEmitterAtLocation` "/Game/VFX/MarketplaceAssets/Realistic_Starter_VFX_Pack_Vol2/Particles/Blood/P_Blood_Splat_Cone_Original.P_Blood_Splat_Cone_Original" (`SceneComponent.K2_GetComponentLocation` _staticmesh) (`SceneComponent.K2_GetComponentRotation` _staticmesh) (`KismetMathLibrary.MakeVector` (`KismetMathLibrary.RandomFloatInRange` 0.7 1.0) (`KismetMathLibrary.RandomFloatInRange` 0.7 1.0) (`KismetMathLibrary.RandomFloatInRange` 0.7 1.0))))
      (`PrimitiveComponent.AddImpulse` (`self.StaticMesh`) (* (`SceneComponent.GetForwardVector` _returnvalue) (`KismetMathLibrary.RandomFloatInRange` 0.0 5000.0)) "None" false)
      (if (`self.Frozen`)
        _
        (elif (`self.RecentlyGibbed`)
          (goto _label)
          (else
            (`KismetSystemLibrary.Delay` (`KismetMathLibrary.RandomFloatInRange` 2.0 5.0))
            (goto _label)))))
    (:`then_2`
      (`KismetSystemLibrary.DelayUntilNextTick`)
      (if (`self.Frozen`)
        (`PrimitiveComponent.SetMaterial` _staticmesh_2 0 "/Game/Materials/IceTexture_Mat.IceTexture_Mat")
        (`PrimitiveComponent.SetMaterial` _staticmesh_2 1 "/Game/Materials/IceTexture_Mat.IceTexture_Mat")))))

(event `self.ReceiveActorBeginOverlap`
  (params (OtherActor :type "Actor Object Reference"))
  (bind _staticmesh (`self.StaticMesh`))
  (bind _returnvalue (`SceneComponent.GetComponentVelocity` (`self.StaticMesh`)))
  (bind _returnvalue_2 (`KismetMathLibrary.VSize` (* _returnvalue 0.05)))
  (bind _asbp_cannonball (cast `/Game/Blueprints/Interactibles/BP_Cannonball` OtherActor)
    (:`then`
      (`/Engine/EditorBlueprintResources/StandardMacros.IsValid` _asbp_cannonball
        (:`Is Valid`
          (`/Game/Blueprints/Interactibles/BP_Cannonball.Explode` _asbp_cannonball))
        (:`Is Not Valid`
          _)))
    (:`CastFailed`
      _))
  (if (not (== _returnvalue (0.0 0.0 0.0) :`ErrorTolerance` 1200.0))
    (cast `Pawn` OtherActor)
    (if (`self.Electrified`)
      (`GameplayStatics.ApplyDamage` OtherActor (/ _returnvalue_2 10.0) null self "/Game/Blueprints/HeathNDamage/DamageType_Lightning.DamageType_Lightning_C"))
    (`GameplayStatics.ApplyDamage` OtherActor _returnvalue_2 null self)
    (`KismetSystemLibrary.DelayUntilNextTick`)
    (`PrimitiveComponent.SetAllPhysicsLinearVelocity` (`self.StaticMesh`) (* (* (`SceneComponent.GetForwardVector` _staticmesh) (/ (`KismetMathLibrary.VSize` (`SceneComponent.GetComponentVelocity` _staticmesh)) 3.0)) -1.0) false)
    (`PrimitiveComponent.AddAngularImpulseInDegrees` (`self.StaticMesh`) (* (`KismetMathLibrary.RandomUnitVector`) 500.0) "None" true)))

(event `self.ReceiveAnyDamage`
  (params (Damage :type "Float (single-precision)") (DamageType :type "DamageType Object Reference") (InstigatedBy :type "Controller Object Reference") (DamageCauser :type "Actor Object Reference"))
  (bind _returnvalue (`self.GetTransform`))
  (bind _forcestorage (`self.ForceStorage`))
  (if (== (`GameplayStatics.GetObjectClass` DamageType) "/Game/Blueprints/HeathNDamage/DamageType_ReturnToPlayer.DamageType_ReturnToPlayer_C")
    (bind _returnvalue_2 (`|SpawnActorFromClass` "/Game/Blueprints/Projectiles/BP_SwordProjectile.BP_SwordProjectile_C" (`KismetMathLibrary.MakeTransform` (.location _returnvalue) (`KismetMathLibrary.MakeRotator` (.roll (.rotation _returnvalue)) (.pitch (.rotation _returnvalue)) (.yaw (.rotation _returnvalue))) (.scale _returnvalue)) "AlwaysSpawn" "MultiplyWithRoot" null 0.1 true (0.0 0.0 3000.0) false false false false (struct) (struct :`Pitch` -90.0 :`Yaw` 720.000927 :`Roll` 1079.99907) true (10000.0 10000.0 0.0) false false null false null false false null 1.0 2.0 false 2 200.0 null))
    (`StaticMeshComponent.SetStaticMesh` (`/Game/Blueprints/Projectiles/BP_SwordProjectile.Greatsword` _returnvalue_2) (`StaticMeshComponent.StaticMesh` (`self.StaticMesh`)))
    (`self.K2_DestroyActor`)
    (elif (== (`GameplayStatics.GetObjectClass` DamageType) "/Game/Blueprints/HeathNDamage/DamageType_Lightning.DamageType_Lightning_C")
      (`|ExecutionSequence`
        (:`then_0`
          (set `self.Electrified` true)
          (`KismetSystemLibrary.RetriggerableDelay` 5.0)
          (set `self.Electrified` false)
          (`/Engine/EditorBlueprintResources/StandardMacros.DoOnce` false :!label _label_2
            (:`Completed`
              (`ActorComponent.Deactivate` (`self.ParticleSystem`))
              (goto _label_3 :!via `Reset`))))
        (:`then_1`
          (`/Engine/EditorBlueprintResources/StandardMacros.DoOnce` false :!label _label_3
            (:`Completed`
              (`ActorComponent.Activate` (`self.ParticleSystem`) true)
              (goto _label_2 :!via `Reset`)))))
      (else
        (set `self.ForceStorage` Damage)
        (`PhysicsObjectBlueprintLibrary.ApplyRadialImpulse` (`self.StaticMesh`) (`self.K2_GetActorLocation` DamageCauser) (* _forcestorage 600.0) (* _forcestorage 80.0) "RIF_Constant")
        (`GameplayStatics.SpawnEmitterAtLocation` "/Game/VFX/Bonuses/P_BulletImpact_Meat.P_BulletImpact_Meat" (`SceneComponent.K2_GetComponentLocation` (`self.StaticMesh`)) (`KismetMathLibrary.RandomRotator` false) (0.1 0.1 0.1))))))

(fn `UserConstructionScript`)