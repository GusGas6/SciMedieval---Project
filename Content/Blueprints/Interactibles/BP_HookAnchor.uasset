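; BP_HookAnchor is a grapple anchor that reels the first-person player toward itself.
; While hooked, a per-tick loop rotates the anchor and relaunches the player at it, with a runtime cable drawn to the player's robot arm.
; When destroyed, it removes the cable and spawns a replacement carrying the hooked state, which launches an overlapping player once with a configurable velocity.
; Anchors flagged hidden hide their sphere.
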(event `self.ReceiveBeginPlay`
  (if (`self.Hidden`)
    (`SceneComponent.SetVisibility` (`self.Sphere`) false false)))

(event `HookToPlayer`
  (bind _returnvalue (`GameplayStatics.GetPlayerCharacter` 0))
  (bind _returnvalue_2 (`self.K2_GetActorLocation`))
  (bind _returnvalue_3 (`self.K2_GetActorLocation` _returnvalue))
  (set `self.NextActorJustHooked` true)
  (set `self.RotatingTowardsPlayer` true)
  (bind _asfirst_person_character (cast `/Game/Blueprints/FirstPersonCharacter` (`GameplayStatics.GetPlayerCharacter` 0)))
  (`/Game/Blueprints/FirstPersonCharacter.HookToAnchor` _asfirst_person_character self)
  (`|ExecutionSequence`
    (:`then_0`
      (if (`self.RotatingTowardsPlayer`) :!label _label
        (`self.K2_SetActorRotation` (`KismetMathLibrary.Conv_VectorToRotator` (`KismetMathLibrary.GetDirectionUnitVector` _returnvalue_3 _returnvalue_2)))
        (`Character.LaunchCharacter` _returnvalue (* (`KismetMathLibrary.GetDirectionUnitVector` _returnvalue_3 _returnvalue_2) 9000.0) true true)
        (`KismetSystemLibrary.DelayUntilNextTick`)
        (goto _label)))
    (:`then_1`
      (bind _returnvalue_4 (`AddComponent|NODE_AddCableComponent-0` :`RelativeTransform` (`KismetMathLibrary.MakeTransform` (`self.K2_GetActorLocation`))))
      (set `CableComponent.EndLocation` (0.0 0.0 0.0) _returnvalue_4)
      (`SceneComponent.SetWorldScale3D` _returnvalue_4 (0.5 0.5 0.5))
      (`SceneComponent.K2_AttachToComponent` _returnvalue_4 (`self.Sphere`) "None" "SnapToTarget" "KeepWorld" "KeepWorld" true)
      (bind _asfirst_person_character_2 (cast `/Game/Blueprints/FirstPersonCharacter` (`GameplayStatics.GetPlayerCharacter` 0)))
      (`CableComponent.SetAttachEndToComponent` _returnvalue_4 (`/Game/Blueprints/FirstPersonCharacter.ScuffedRobotArm` _asfirst_person_character_2) "None")
      (`/Engine/EditorBlueprintResources/StandardMacros.IsValid` _returnvalue_4
        (:`Is Valid`
          (`PrimitiveComponent.SetMaterial` _returnvalue_4 0 "/Game/CustomMaterials/MI_Template_DarkMetal.MI_Template_DarkMetal"))))))

(event `UnhookFromPlayer`
  (set `self.RotatingTowardsPlayer` false)
  (`/Engine/EditorBlueprintResources/StandardMacros.IsValid` (stale `HookToPlayer` _returnvalue_4) :!label _label_2
    (:`Is Valid`
      (`ActorComponent.K2_DestroyComponent` (stale `HookToPlayer` _returnvalue_4)))))

(event `self.ReceiveDestroyed`
  (`|SpawnActorFromClass` "BP_HookAnchor_C" (`self.GetTransform`) "Undefined" "MultiplyWithRoot" null (`self.Hidden`) (`self.NextActorJustHooked`) null)
  (goto _label_2))

(event `self.ReceiveActorBeginOverlap`
  (params (OtherActor :type "Actor Object Reference"))
  (bind _asfirst_person_character (cast `/Game/Blueprints/FirstPersonCharacter` OtherActor))
  (if (`self.JustHooked`)
    (`/Engine/EditorBlueprintResources/StandardMacros.DoOnce` false
      (:`Completed`
        (`Character.LaunchCharacter` _asfirst_person_character (`self.Launch Velocity`) true true)))))

(fn `UserConstructionScript`)