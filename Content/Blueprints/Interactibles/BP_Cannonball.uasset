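; BP_Cannonball is a physical explosive that spawns a BP_AoEBubble and scorch decal, with frost or lightning material variants.
; Shotgun, lightning or non-player damage detonates it, while other player hits shove it by radial impulse.
; Fast overlaps also detonate it, and other blasts chain-trigger it after a random delay.
; Player-spawned balls explode on nearby targets or a timed fuse; holding one blocks detonation.
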(event `self.ReceiveBeginPlay`
  (bind _explosion_damage_type (`self.Explosion Damage Type`))
  (bind _truebombmesh (`self.TrueBombMesh`))
  (if (== _explosion_damage_type "/Game/Blueprints/HeathNDamage/DamageType_Ice.DamageType_Ice_C")
    (`PrimitiveComponent.SetMaterial` _truebombmesh 0 "/Game/CustomMaterials/Frost_Explosive_Mat.Frost_Explosive_Mat")
    (elif (== _explosion_damage_type "/Game/Blueprints/HeathNDamage/DamageType_Lightning.DamageType_Lightning_C")
      (`PrimitiveComponent.SetMaterial` _truebombmesh 0 "/Game/CustomMaterials/Lightning_Explosive_Mat.Lightning_Explosive_Mat")))
  (if (`self.SpawnFromPlayer`)
    (`PrimitiveComponent.SetCollisionResponseToChannel` (`self.TrueBombMesh`) "ECC_GameTraceChannel2" "ECR_Ignore")
    (bind _asfirst_person_character (cast `/Game/Blueprints/FirstPersonCharacter` (`GameplayStatics.GetPlayerCharacter` 0)))
    (bind (_outactors _returnvalue) (`KismetSystemLibrary.SphereOverlapActors` (`SceneComponent.K2_GetComponentLocation` (`self.TrueBombMesh`)) 50.0 (`|MakeArray` "ObjectTypeQuery6" "ObjectTypeQuery3" :!type "EObjectTypeQuery Enum") null (`|MakeArray` _asfirst_person_character self :!type "Actor Object Reference")))
    (if _returnvalue
      (for _ _outactors
        (`/Engine/EditorBlueprintResources/StandardMacros.DoOnce` false
          (:`Completed`
            (`self.Explode`)))))
    (`KismetSystemLibrary.Delay` 3.0)
    (`self.Explode`)))

(event `self.ReceiveAnyDamage`
  (params (Damage :type "Float (single-precision)") (DamageType :type "DamageType Object Reference") (InstigatedBy :type "Controller Object Reference") (DamageCauser :type "Actor Object Reference"))
  (bind _forcestorage (`self.ForceStorage`))
  (`|ExecutionSequence`
    (:`then_0`
      (if (== (`GameplayStatics.GetObjectClass` DamageType) "/Game/Blueprints/HeathNDamage/DamageType_Shotgun.DamageType_Shotgun_C")
        (if (not (`self.HeldByPlayer`)) :!label _label
          (set `self.Area Of Effect Radius` 350.0)
          (`self.Explode`))
        (elif (== (`GameplayStatics.GetObjectClass` DamageType) "/Game/Blueprints/HeathNDamage/DamageType_Lightning.DamageType_Lightning_C")
          (goto _label)
          (else
            (set `self.ForceStorage` Damage)
            (`PhysicsObjectBlueprintLibrary.ApplyRadialImpulse` (`self.TrueBombMesh`) (`self.K2_GetActorLocation` DamageCauser) (* _forcestorage 60.0) (* _forcestorage 100.0) "RIF_Constant")
            (`GameplayStatics.SpawnEmitterAtLocation` "/Game/VFX/Bonuses/P_BulletImpact_Meat.P_BulletImpact_Meat" (`SceneComponent.K2_GetComponentLocation` (`self.TrueBombMesh`)) (`KismetMathLibrary.RandomRotator` false) (0.1 0.1 0.1))
            (cast `/Game/Blueprints/FirstPersonCharacter` DamageCauser
              (:`CastFailed`
                (`|ExecutionSequence`
                  (:`then_0`
                    (cast `/Game/Blueprints/Projectiles/BP_SwordProjectile` DamageCauser
                      (:`then`
                        (`self.Explode`))
                      (:`CastFailed`
                        (cast `/Game/Blueprints/HeathNDamage/BP_AoEBubble` DamageCauser)
                        (`self.Explode`))))
                  (:`then_1`
                    (`KismetSystemLibrary.Delay` 0.05)
                    (set `self.Primed` true)
                    (if (== (`SceneComponent.GetComponentVelocity` (`self.TrueBombMesh`)) (0.0 0.0 0.0) :`ErrorTolerance` 200.0) :!label _label_2
                      (set `self.Primed` false)
                      (else
                        (`KismetSystemLibrary.Delay` 0.1)
                        (goto _label_2))))
                  (:`then_2`
                    (`self.Explode`)))))))))
    (:`then_1`
      (if (== (`GameplayStatics.GetObjectClass` DamageType) "/Game/Blueprints/HeathNDamage/DamageType_Blunt.DamageType_Blunt_C")
        (set `self.Min` 0.0)
        (set `self.Max` 0.0)))))

(event `Explode`
  (bind _returnvalue (`SceneComponent.K2_GetComponentLocation` (`self.TrueBombMesh`)))
  (`ActorComponent.Activate` (`self.ParticleSystem`) false)
  (if (not (`self.SpawnFromPlayer`))
    (`KismetSystemLibrary.Delay` (`KismetMathLibrary.RandomFloatInRange` (`self.Min`) (`self.Max`)) :!label _label_3))
  (if (not (`self.HeldByPlayer`)) :!label _label_4
    (`/Engine/EditorBlueprintResources/StandardMacros.DoOnce` false
      (:`Completed`
        (`|SpawnActorFromClass` "/Game/Blueprints/HeathNDamage/BP_AoEBubble.BP_AoEBubble_C" (`KismetMathLibrary.MakeTransform` (`SceneComponent.K2_GetComponentLocation` (`self.TrueBombMesh`))) "Undefined" "MultiplyWithRoot" null (`self.Area Of Effect Radius`) (`self.Ao EDamage`) (`self.Explosion?`) (`self.Show Debug Sphere`) (`self.Explosion Knockback Force`) (`self.Explosion Damage Type`) null)
        (bind (_outhit _returnvalue_2) (`KismetSystemLibrary.LineTraceSingleForObjects` _returnvalue (- _returnvalue (0.0 0.0 250.0)) (`|MakeArray` "ObjectTypeQuery1" :!type "EObjectTypeQuery Enum")))
        (if _returnvalue_2
          (bind (_bblockinghit _binitialoverlap _time _distance _location _impactpoint _normal) (`GameplayStatics.BreakHitResult` _outhit))
          (`|SpawnActorFromClass` "/Game/Blueprints/Lighting/BP_ScorchDecal.BP_ScorchDecal_C" (`KismetMathLibrary.MakeTransform` _location (`KismetMathLibrary.MakeRotFromZ` _normal) (2.0 2.0 2.0)) "AlwaysSpawn" "MultiplyWithRoot" null null))
        (`self.K2_DestroyActor`)))))

(event `self.ReceiveActorBeginOverlap`
  (params (OtherActor :type "Actor Object Reference"))
  (cast `/Game/Blueprints/BP_ThirdPersonCharacter` OtherActor
    (:`CastFailed`
      (cast `/Game/Blueprints/HeathNDamage/BP_AoEBubble` OtherActor
        (:`then`
          (goto _label_3))
        (:`CastFailed`
          (if (not (== (`SceneComponent.GetComponentVelocity` (`self.TrueBombMesh`)) (0.0 0.0 0.0) :`ErrorTolerance` 600.0))
            (goto _label_4)))))))

(fn `UserConstructionScript`)