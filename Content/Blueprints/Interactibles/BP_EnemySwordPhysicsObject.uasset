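; A loose physics sword that can be knocked around, hurt pawns, and be recalled to the player as a weapon.
; Fast overlaps deal speed-scaled damage and rebound the sword with spin; touched cannonballs explode.
; Damage type acts as a command: return-to-player swaps it for a returning BP_SwordProjectile carrying its mesh and stats, lightning temporarily electrifies it for bonus damage, other hits apply impulses.
; Collision and kicking enable shortly after spawn.
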(event `self.ReceiveBeginPlay`
  (`KismetSystemLibrary.Delay` 0.5)
  (`PrimitiveComponent.SetCollisionEnabled` (`self.PhysicsSwordBox`) "QueryAndPhysics")
  (set `self.CannotBeKicked` false))

(event `self.PhysicsSwordBox.OnComponentBeginOverlap`
  (params (OverlappedComponent :type "PrimitiveComponent Object Reference") (OtherActor :type "Actor Object Reference") (OtherComp :type "PrimitiveComponent Object Reference") (OtherBodyIndex :type Integer) (bFromSweep :type Boolean) (SweepResult :type "HitResult Structure (by ref)"))
  (bind _physicssword (`self.PhysicsSword`))
  (bind _returnvalue (`SceneComponent.GetComponentVelocity` (`self.PhysicsSword`)))
  (bind _returnvalue_2 (`KismetMathLibrary.VSize` (* _returnvalue 0.05)))
  (bind _asbp_cannonball (cast `/Game/Blueprints/Interactibles/BP_Cannonball` OtherActor)
    (:`then`
      (`/Game/Blueprints/Interactibles/BP_Cannonball.Explode` _asbp_cannonball))
    (:`CastFailed`
      _))
  (if (not (== _returnvalue (0.0 0.0 0.0) :`ErrorTolerance` 1200.0))
    (cast `Pawn` OtherActor)
    (if (`self.Electrified`)
      (`GameplayStatics.ApplyDamage` OtherActor (/ _returnvalue_2 10.0) null self "/Game/Blueprints/HeathNDamage/DamageType_Lightning.DamageType_Lightning_C"))
    (`GameplayStatics.ApplyDamage` OtherActor _returnvalue_2 null self)
    (`KismetSystemLibrary.DelayUntilNextTick`)
    (`PrimitiveComponent.SetAllPhysicsLinearVelocity` (`self.PhysicsSword`) (* (* (`SceneComponent.GetForwardVector` _physicssword) (/ (`KismetMathLibrary.VSize` (`SceneComponent.GetComponentVelocity` _physicssword)) 3.0)) -1.0) false)
    (`PrimitiveComponent.AddAngularImpulseInDegrees` (`self.PhysicsSword`) (* (`KismetMathLibrary.RandomUnitVector`) 500.0) "None" true)))

(event `self.ReceiveAnyDamage`
  (params (Damage :type "Float (single-precision)") (DamageType :type "DamageType Object Reference") (InstigatedBy :type "Controller Object Reference") (DamageCauser :type "Actor Object Reference"))
  (bind _forcestorage (`self.ForceStorage`))
  (bind _staticmesh (`StaticMeshComponent.StaticMesh` (`self.PhysicsSword`)))
  (`PrimitiveComponent.SetSimulatePhysics` (`self.PhysicsSword`) true)
  (if (== (`GameplayStatics.GetObjectClass` DamageType) "/Game/Blueprints/HeathNDamage/DamageType_ReturnToPlayer.DamageType_ReturnToPlayer_C")
    (bind _asfirst_person_character (cast `/Game/Blueprints/FirstPersonCharacter` (`GameplayStatics.GetPlayerCharacter` 0)))
    (set `/Game/Blueprints/FirstPersonCharacter.WeaponIsReturning` true _asfirst_person_character)
    (bind _returnvalue (`|SpawnActorFromClass` "/Game/Blueprints/Projectiles/BP_SwordProjectile.BP_SwordProjectile_C" (`self.GetTransform`) "AlwaysSpawn" "MultiplyWithRoot" null 0.1 true (0.0 0.0 3000.0) false false false false (struct) (struct :`Pitch` -90.0 :`Yaw` 720.000927 :`Roll` 1079.99907) true (10000.0 10000.0 0.0) (`self.BluntWeapon`) false null true null false false (`self.ThrownSwordDamageType`) (`self.BaseGlobalAnimRate`) (`self.ChargedGlobalAnimRate`) false (`self.Weapon Size`) (`self.Base Damage Sword`) null))
    (bind _greatsword (`/Game/Blueprints/Projectiles/BP_SwordProjectile.Greatsword` _returnvalue))
    (`SceneComponent.K2_SetWorldTransform` _greatsword (`SceneComponent.K2_GetComponentToWorld` (`self.PhysicsSword`)) false false)
    (if (== _staticmesh "BP_EnemySwordPhysicsObject")
      (`StaticMeshComponent.SetStaticMesh` _greatsword "/Game/Models/Weapons/SM_Sword1.SM_Sword1")
      (`self.K2_DestroyActor`)
      (else
        (`StaticMeshComponent.SetStaticMesh` _greatsword _staticmesh)
        (`self.K2_DestroyActor`)))
    (elif (== (`GameplayStatics.GetObjectClass` DamageType) "/Game/Blueprints/HeathNDamage/DamageType_Lightning.DamageType_Lightning_C")
      (`|ExecutionSequence`
        (:`then_0`
          (set `self.Electrified` true)
          (`KismetSystemLibrary.RetriggerableDelay` 5.0)
          (set `self.Electrified` false)
          (`/Engine/EditorBlueprintResources/StandardMacros.DoOnce` false :!label _label
            (:`Completed`
              (`ActorComponent.Deactivate` (`self.ParticleSystem`))
              (goto _label_2 :!via `Reset`))))
        (:`then_1`
          (`/Engine/EditorBlueprintResources/StandardMacros.DoOnce` false :!label _label_2
            (:`Completed`
              (`ActorComponent.Activate` (`self.ParticleSystem`) true)
              (goto _label :!via `Reset`)))))
      (elif (not (`self.CannotBeKicked`))
        (set `self.ForceStorage` Damage)
        (`PhysicsObjectBlueprintLibrary.ApplyRadialImpulse` (`self.PhysicsSword`) (`self.K2_GetActorLocation` DamageCauser) (* _forcestorage 600.0) (* _forcestorage 600.0) "RIF_Constant")
        (`GameplayStatics.SpawnEmitterAtLocation` "/Game/VFX/Bonuses/P_BulletImpact_Meat.P_BulletImpact_Meat" (`SceneComponent.K2_GetComponentLocation` (`self.PhysicsSword`)) (`KismetMathLibrary.RandomRotator` false) (0.1 0.1 0.1))))))

(fn `UserConstructionScript`)