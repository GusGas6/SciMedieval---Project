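; BP_TripBox is a physics prop that can be knocked around and hurts what it hits, ignoring the first-person player.
; On overlap, it applies speed-scaled, capped InstaGib damage, then resets its velocity from the direction to the target and its negated velocity, with a brief DoOnce cooldown.
; Taking damage triggers a damage-scaled radial impulse and impact particles, then next tick sets a reduced backward velocity and adds random spin.
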(event `self.ReceiveActorBeginOverlap`
  (params (OtherActor :type "Actor Object Reference"))
  (bind _staticmesh (`self.StaticMesh`))
  (cast `/Game/Blueprints/FirstPersonCharacter` OtherActor
    (:`CastFailed`
      (`GameplayStatics.ApplyDamage` OtherActor (`KismetMathLibrary.FClamp` (* (`KismetMathLibrary.VSize` (`SceneComponent.GetComponentVelocity` (`self.StaticMesh`))) 0.6) 0.0 100.0) null self "/Game/Blueprints/HeathNDamage/DamageType_InstaGib.DamageType_InstaGib_C")
      (`/Engine/EditorBlueprintResources/StandardMacros.IsValid` OtherActor
        (:`Is Valid`
          (`/Engine/EditorBlueprintResources/StandardMacros.DoOnce` false :!label _label
            (:`Completed`
              (`PrimitiveComponent.SetPhysicsLinearVelocity` (`self.StaticMesh`) (* (`KismetMathLibrary.GetDirectionUnitVector` (`SceneComponent.K2_GetComponentLocation` _staticmesh) (`self.K2_GetActorLocation` OtherActor)) (* (`SceneComponent.GetComponentVelocity` _staticmesh) -1.0)) false "None")
              (`KismetSystemLibrary.Delay` 0.2)
              (goto _label :!via `Reset`))))))))

(event `self.ReceiveAnyDamage`
  (params (Damage :type "Float (single-precision)") (DamageType :type "DamageType Object Reference") (InstigatedBy :type "Controller Object Reference") (DamageCauser :type "Actor Object Reference"))
  (bind _forcestorage (`self.ForceStorage`))
  (bind _staticmesh (`self.StaticMesh`))
  (bind _staticmesh_2 (`self.StaticMesh`))
  (set `self.ForceStorage` Damage)
  (`PhysicsObjectBlueprintLibrary.ApplyRadialImpulse` (`self.StaticMesh`) (`self.K2_GetActorLocation` DamageCauser) (* _forcestorage 600.0) (* _forcestorage 2000.0) "RIF_Constant")
  (`GameplayStatics.SpawnEmitterAtLocation` "/Game/VFX/Bonuses/P_BulletImpact_Meat.P_BulletImpact_Meat" (`SceneComponent.K2_GetComponentLocation` (`self.StaticMesh`)) (`KismetMathLibrary.RandomRotator` false) (0.1 0.1 0.1))
  (`KismetSystemLibrary.DelayUntilNextTick`)
  (`PrimitiveComponent.SetAllPhysicsLinearVelocity` _staticmesh_2 (* (* (`SceneComponent.GetForwardVector` _staticmesh) (/ (`KismetMathLibrary.VSize` (`SceneComponent.GetComponentVelocity` _staticmesh)) 3.0)) -1.0) false)
  (`PrimitiveComponent.AddAngularImpulseInDegrees` _staticmesh_2 (* (`KismetMathLibrary.RandomUnitVector`) 500.0) "None" true))

(fn `UserConstructionScript`)