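; Test interactible "glowy door" that appears under the fake lantern light and can be destroyed by the player.
; The mesh starts flattened to zero Y scale; a timeline grows it to full while BP_FakeLanternLightDecal overlaps and reverses when the overlap ends.
; Any damage caused by BP_ThirdPersonCharacter destroys the actor, spawning randomly scaled ghost sparks below the mesh origin.
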(event `self.ReceiveBeginPlay`
  (`SceneComponent.SetWorldScale3D` (`self.StaticMesh`) (1.0 0.0 1.0)))

(event `self.ReceiveActorBeginOverlap`
  (params (OtherActor :type "Actor Object Reference"))
  (cast `/Game/Blueprints/Lighting/BP_FakeLanternLightDecal` OtherActor)
  (bind (_direction _newtrack_0) (`Timeline|Timeline` :!label _label)
    (:`Update`
      (`SceneComponent.SetWorldScale3D` (`self.StaticMesh`) (`KismetMathLibrary.VLerp` (1.0 0.0 1.0) (1.0 1.0 1.0) _newtrack_0)))))

(event `self.ReceiveActorEndOverlap`
  (params (OtherActor :type "Actor Object Reference"))
  (cast `/Game/Blueprints/Lighting/BP_FakeLanternLightDecal` OtherActor)
  (goto _label :!via `Reverse`))

(event `self.ReceiveAnyDamage`
  (params (Damage :type "Float (single-precision)") (DamageType :type "DamageType Object Reference") (InstigatedBy :type "Controller Object Reference") (DamageCauser :type "Actor Object Reference"))
  (cast `/Game/Blueprints/BP_ThirdPersonCharacter` DamageCauser)
  (`self.K2_DestroyActor`))

(event `self.ReceiveDestroyed`
  (bind _returnvalue (`KismetMathLibrary.RandomFloatInRange` 0.8 1.3))
  (bind _staticmesh (`self.StaticMesh`))
  (`GameplayStatics.SpawnEmitterAtLocation` "/Game/MarketplaceAssets/DreamscapeSeries/DreamscapeTower/Effects/P_GhostSparks.P_GhostSparks" (+ (`SceneComponent.K2_GetComponentLocation` _staticmesh) (0.0 0.0 -250.0)) (`SceneComponent.K2_GetComponentRotation` _staticmesh) (`KismetMathLibrary.MakeVector` _returnvalue _returnvalue _returnvalue)))

(fn `UserConstructionScript`)