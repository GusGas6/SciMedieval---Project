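; BP_ForceActor is a short-lived interactible actor that fires a one-shot physics impulse through its ForceComponent.
; On BeginPlay it copies its radius, strength and velocity-change settings onto the component and optionally shows a debug sphere.
; It waits until the next tick to fire the impulse, then destroys itself after a brief delay.
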(event `self.ReceiveBeginPlay`
  (bind _forcecomponent (`self.ForceComponent`))
  (set `RadialForceComponent.bImpulseVelChange` (`self.Impulse Vel Change`) _forcecomponent)
  (set `RadialForceComponent.ImpulseStrength` (`self.Impulse Strength`) _forcecomponent)
  (set `RadialForceComponent.Radius` (`self.Radius`) _forcecomponent)
  (`|ExecutionSequence`
    (:`then_0`
      (if (`self.ShowDebugSphere`)
        (`SceneComponent.SetVisibility` (`self.Sphere`) true false)))
    (:`then_1`
      (`KismetSystemLibrary.DelayUntilNextTick`)
      (`RadialForceComponent.FireImpulse` _forcecomponent)
      (`KismetSystemLibrary.Delay` 0.2)
      (`self.K2_DestroyActor`))))

(fn `UserConstructionScript`)