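; BP_FrozenGround is an ice spell's temporary frozen ground patch that applies slip damage to overlapping actors.
; On spawn it picks one of three decal materials, and a timeline reversed from its end scales it up from zero.
; After a brief arming delay it hits current overlaps except FirstPersonCharacter, then any new overlap.
; When its lifetime expires, particles stop and the patch later shrinks away and is destroyed.
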(event `self.ReceiveBeginPlay`
  (bind _decal (`self.Decal`))
  (set `self.DecalScale` (`self.GetActorScale3D`))
  (switch `int` (`KismetMathLibrary.RandomIntegerInRange` 0 2)
    (:`0`
      (`DecalComponent.SetDecalMaterial` _decal "/Game/Blueprints/MagicSpells/Ice/ice_ground_decal_texture__1__Mat.ice_ground_decal_texture__1__Mat"))
    (:`1`
      (`DecalComponent.SetDecalMaterial` _decal "/Game/Blueprints/MagicSpells/Ice/ice_ground_decal_texture__2__Mat.ice_ground_decal_texture__2__Mat"))
    (:`2`
      (`DecalComponent.SetDecalMaterial` _decal "/Game/Blueprints/MagicSpells/Ice/ice_ground_decal_texture__3__Mat.ice_ground_decal_texture__3__Mat")))
  (`|ExecutionSequence`
    (:`then_0`
      (`self.SetActorScale3D` (* (`self.GetActorScale3D`) (`KismetMathLibrary.RandomFloatInRange` 0.7 1.0)))
      (`KismetSystemLibrary.Delay` (`self.customdecallifetime`))
      (`ActorComponent.Deactivate` (`self.PS_FX_particle_windtrail`))
      (`KismetSystemLibrary.Delay` 10.0)
      (`|ExecutionSequence`
        (:`then_0`
          (`KismetSystemLibrary.Delay` 0.3)
          (`self.K2_DestroyActor`))
        (:`then_1`
          (bind (_direction _newtrack_0) (`Timeline|Timeline_0` :!via `PlayFromStart` :!label _label)
            (:`Update`
              (`self.SetActorScale3D` (`KismetMathLibrary.VLerp` (`self.DecalScale`) (0.0 0.0 0.0) _newtrack_0)))))))
    (:`then_1`
      (goto _label :!via `ReverseFromEnd`))
    (:`then_2`
      (`KismetSystemLibrary.Delay` 0.3)
      (set `self.ReadyToSlip` true)
      (for _array_element (`PrimitiveComponent.GetOverlappingActors` (`self.Box`) null)
        (cast `/Game/Blueprints/FirstPersonCharacter` _array_element
          (:`CastFailed`
            (`GameplayStatics.ApplyDamage` _array_element 0.01 null self "/Game/Blueprints/HeathNDamage/DamageType_Slippy.DamageType_Slippy_C")))))))

(event `self.ReceiveActorBeginOverlap`
  (params (OtherActor :type "Actor Object Reference"))
  (if (`self.ReadyToSlip`)
    (`GameplayStatics.ApplyDamage` OtherActor 0.01 null self "/Game/Blueprints/HeathNDamage/DamageType_Slippy.DamageType_Slippy_C")))

(fn `UserConstructionScript`
  (`parent.UserConstructionScript`))