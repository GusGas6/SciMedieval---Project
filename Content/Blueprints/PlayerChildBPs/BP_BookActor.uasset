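; BP_BookActor is a book prop that swings open on BeginPlay and exposes events to close it slowly, quickly for a smack, or instantly.
; A timeline lerps the StaticMesh rotation to open it and reverses to close it, with CustomTimeDilation speeding up the smack close.
; A second timeline nudges the Plane's yaw incrementally from its current value, calling Play again when finished.
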(event `self.ReceiveBeginPlay`
  (bind _plane (`self.Plane`))
  (bind (_relativerotation_roll _relativerotation_pitch _relativerotation_yaw) (`KismetMathLibrary.BreakRotator` (`SceneComponent.RelativeRotation` _plane)))
  (`/Engine/EditorBlueprintResources/StandardMacros.DoOnce` false
    (:`Completed`
      (`|ExecutionSequence`
        (:`then_0`
          (bind (_direction _newtrack_0) (`Timeline|Timeline_0` :!via `PlayFromStart` :!label _label)
            (:`Update`
              (`SceneComponent.K2_SetRelativeRotation` _plane (`KismetMathLibrary.RLerp` (`KismetMathLibrary.MakeRotator` _relativerotation_roll _relativerotation_pitch _relativerotation_yaw) (`KismetMathLibrary.MakeRotator` _relativerotation_roll _relativerotation_pitch (+ _relativerotation_yaw 0.3)) _newtrack_0) false false))
            (:`Finished`
              (`KismetSystemLibrary.Delay` 0.0)
              (goto _label))))
        (:`then_1`
          (`self.OpenBook`))))))

(event `OpenBook`
  (set `self.CustomTimeDilation` 1.0)
  (bind (_direction _newtrack_0) (`Timeline|Timeline` :!via `PlayFromStart` :!label _label_2)
    (:`Update`
      (`SceneComponent.K2_SetRelativeRotation` (`self.StaticMesh`) (`KismetMathLibrary.RLerp` (struct) (struct :`Roll` 160.0) _newtrack_0) false false))
    (:`Finished`
      (set `self.CustomTimeDilation` 1.0))))

(event `CloseBookSlow`
  (set `self.CustomTimeDilation` 1.0)
  (goto _label_2 :!via `ReverseFromEnd`))

(event `CloseBookForSmack`
  (set `self.CustomTimeDilation` 3.0)
  (goto _label_2 :!via `ReverseFromEnd`))

(event `CloseBook`
  (`|ExecutionSequence`
    (:`then_0`
      (set `self.CustomTimeDilation` 1.0)
      (goto _label_2 :!via `Stop`))
    (:`then_1`
      (`KismetSystemLibrary.DelayUntilNextTick`)
      (`SceneComponent.K2_SetRelativeRotation` :`self` (`self.StaticMesh`)))))

(fn `UserConstructionScript`)