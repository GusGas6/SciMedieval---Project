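; Blueprint that fakes flickering brazier light with a decal and a sphere, using an orange or light blue torchlight material, or a blob shadow variant.
; BeginPlay picks the decal material and records the sphere's initial XY scale length.
; A randomized delay loop compares current scale to that baseline, choosing a higher or lower random multiplier around BaseSize.
; A replayed timeline lerps the sphere's scale with that multiplier to create the flicker.
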(event `self.ReceiveBeginPlay`
  (bind _basesize (`self.BaseSize`))
  (bind _basesize_2 (`self.BaseSize`))
  (bind _sphere (`self.Sphere`))
  (bind _decal (`self.Decal`))
  (bind _basesize_3 (`self.BaseSize`))
  (bind _relativescale3d (`SceneComponent.RelativeScale3D` _sphere))
  (set `self.InitialVectorLength` (`KismetMathLibrary.VSizeXY` (`SceneComponent.RelativeScale3D` (`self.Sphere`))))
  (if (`self.BlobShadow`)
    (`DecalComponent.SetDecalMaterial` _decal "/Game/CustomMaterials/FakeLighting/fakeblobshadow_mat.fakeblobshadow_mat")
    (elif (`self.Orange`)
      (`DecalComponent.SetDecalMaterial` _decal "/Game/CustomMaterials/FakeLighting/faketorchlighttest_Mat.faketorchlighttest_Mat")
      (else
        (`DecalComponent.SetDecalMaterial` _decal "/Game/CustomMaterials/FakeLighting/faketorchlight_lightblue_mat.faketorchlight_lightblue_mat"))))
  (`|ExecutionSequence`
    (:`then_0`
      (`KismetSystemLibrary.Delay` (`KismetMathLibrary.RandomFloatInRange` 0.2 0.28) :!label _label)
      (`|ExecutionSequence`
        (:`then_0`
          (goto _label))
        (:`then_1`
          (if (<= (`KismetMathLibrary.VSizeXY` (`SceneComponent.RelativeScale3D` (`self.Sphere`))) (`self.InitialVectorLength`))
            (set `self.SetRandomFakeLightRange` (`KismetMathLibrary.RandomFloatInRange` (+ _basesize_2 0.005) (+ _basesize_2 0.015)))
            (bind (_direction _newtrack_0) (`Timeline|Timeline` :!via `PlayFromStart` :!label _label_2)
              (:`Update`
                (`SceneComponent.SetRelativeScale3D` _sphere (`KismetMathLibrary.VLerp` (* _relativescale3d (`self.SetRandomFakeLightRange`)) _relativescale3d _newtrack_0))))
            (else
              (set `self.SetRandomFakeLightRange` (`KismetMathLibrary.RandomFloatInRange` (- _basesize 0.01) (- _basesize 0.005)))
              (goto _label_2 :!via `PlayFromStart`))))))
    (:`then_1`
      (set `self.SetRandomFakeLightRange` (`KismetMathLibrary.RandomFloatInRange` (+ _basesize_3 -0.005) (+ _basesize_3 0.095)))
      (goto _label_2 :!via `PlayFromStart`))))

(fn `UserConstructionScript`)