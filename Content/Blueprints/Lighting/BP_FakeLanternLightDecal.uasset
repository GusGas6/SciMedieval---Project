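; Fake lantern light actor that pairs a Sphere with a Decal held at a fixed world rotation every Tick.
; On BeginPlay a timeline scales the Sphere up from zero to full size.
; Unequip reverses that timeline to shrink the Sphere, then destroys the actor after a short delay.
; A randomized looping flicker that would nudge the Sphere's scale around a base size is present but disconnected, so it never runs.
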(event `self.ReceiveTick`
  (params (DeltaSeconds :type "Float (single-precision)"))
  (`SceneComponent.K2_SetWorldRotation` (`self.Decal`) (struct :`Pitch` 90.0) false false))

(event `self.ReceiveBeginPlay`
  (bind (_direction _newtrack_0) (`Timeline|Timeline_0` :!label _label)
    (:`Update`
      (`SceneComponent.SetRelativeScale3D` (`self.Sphere`) (`KismetMathLibrary.VLerp` (0.0 0.0 0.0) (1.0 1.0 1.0) _newtrack_0)))))

(event `Unequip`
  (`|ExecutionSequence`
    (:`then_0`
      (goto _label :!via `Reverse`))
    (:`then_1`
      (`KismetSystemLibrary.Delay` 1.0)
      (`self.K2_DestroyActor`))))

(fn `UserConstructionScript`)