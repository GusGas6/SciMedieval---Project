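; BP_ScorchDecal is a self-removing scorch decal actor with a wind-trail particle effect.
; On BeginPlay it randomizes its yaw and scale for variation, then waits a configurable lifetime before deactivating the particles.
; After a further fixed delay, a timeline shrinks it by repeatedly lerping its current scale toward zero, then destroys the actor.
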(event `self.ReceiveBeginPlay`
  (bind (_returnvalue_roll _returnvalue_pitch) (`KismetMathLibrary.BreakRotator` (`self.K2_GetActorRotation`)))
  (`self.K2_SetActorRotation` (`KismetMathLibrary.MakeRotator` _returnvalue_roll _returnvalue_pitch (`KismetMathLibrary.RandomFloatInRange` -720.0 720.0)))
  (`self.SetActorScale3D` (* (`self.GetActorScale3D`) (`KismetMathLibrary.RandomFloatInRange` 0.7 1.0)))
  (`KismetSystemLibrary.Delay` (`self.customdecallifetime`))
  (`ActorComponent.Deactivate` (`self.PS_FX_particle_windtrail`))
  (`KismetSystemLibrary.Delay` 35.0)
  (bind (_direction _newtrack_0) (`Timeline|Timeline` :!via `PlayFromStart`)
    (:`Update`
      (`self.SetActorScale3D` (`KismetMathLibrary.VLerp` (`self.GetActorScale3D`) (0.0 0.0 0.0) _newtrack_0)))
    (:`Finished`
      (`self.K2_DestroyActor`))))

(fn `UserConstructionScript`)